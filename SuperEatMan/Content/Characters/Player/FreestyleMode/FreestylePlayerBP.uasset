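; FreestylePlayerBP is the player Blueprint for Freestyle mode, adding a HUD with a damage indicator on top of its parent class.
; On BeginPlay it creates the WB_FreestyleUI widget, adds it to the viewport and hides its PlayerHit element.
; SEMDamaged shows PlayerHit for DamageDelay seconds, using a DoOnce that resets afterward so repeated hits during that window are ignored.
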(event `self.ReceiveBeginPlay`
  (`parent.ReceiveBeginPlay`)
  (bind _returnvalue (`|CreateWidget` "/Game/Characters/Player/FreestyleMode/WB_FreestyleUI.WB_FreestyleUI_C"))
  (bind _output_get (set `self.FreeStyleUI` _returnvalue))
  (`UserWidget.AddToViewport` _output_get 0)
  (`Widget.SetVisibility` (`/Game/Characters/Player/FreestyleMode/WB_FreestyleUI.PlayerHit` (`self.FreeStyleUI`)) "Hidden"))

(event `self.SEM Damaged`
  (`/Engine/EditorBlueprintResources/StandardMacros.DoOnce` false :!label _label ; After this, put code to tell player they were damaged
    (:`Completed`
      (`Widget.SetVisibility` (`/Game/Characters/Player/FreestyleMode/WB_FreestyleUI.PlayerHit` (`self.FreeStyleUI`)) "Visible")
      (`KismetSystemLibrary.Delay` (`self.DamageDelay`))
      (`Widget.SetVisibility` (`/Game/Characters/Player/FreestyleMode/WB_FreestyleUI.PlayerHit` (`self.FreeStyleUI`)) "Hidden")
      (goto _label :!via `Reset`))))

(fn `UserConstructionScript`
  (`parent.UserConstructionScript`))