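; BP_Guardie is an enemy NPC that flies a spline path while firing lasers.
; It takes the path from its parent BP_GuardieSpline and moves along it on a timeline, deriving rotation from a look-at toward the player.
; A DoOnce and Delay on Tick repeatedly fire BP_GuardieLaser from three source points; the spread checks are empty.
; Each hit removes one HP, and death destroys both the Guardie and its spline.
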(event `self.ReceiveBeginPlay`
  (bind _asbp_guardie_spline (cast `/Game/Characters/NPC/Enemies/Guardie/BP_GuardieSpline` (`self.GetParentActor`)))
  (set `self.SplineRef` _asbp_guardie_spline)
  (`self.Move Object`))

(event `self.ReceiveTick`
  (params (DeltaSeconds :type "Float (single-precision)"))
  (`/Engine/EditorBlueprintResources/StandardMacros.DoOnce` false :!label _label
    (:`Completed`
      (`self.Shoot` 0.0)
      (`KismetSystemLibrary.Delay` 5.0)
      (goto _label :!via `Reset`))))

(event `Shoot`
  (params (SpreadIntensity :type "Float (double-precision)"))
  (if (> SpreadIntensity (`self.MaxSpread`))
    _
    (else
      _))
  (if (<= SpreadIntensity (`self.MinSpread`))
    _
    (else
      _))
  (`self.FireSingle` (`self.ProjectSrcCenter`))
  (`self.FireSingle` (`self.ProjectSrcRight`))
  (`self.FireSingle` (`self.ProjectSrcLeft`)))

(event `Move Object`
  (bind _spline (`/Game/Characters/NPC/Enemies/Guardie/BP_GuardieSpline.Spline` (`self.SplineRef`)))
  (`TimelineComponent.SetPlayRate` (`self.Move Object T`) (/ 1.0 (`self.TimeToComplete`)))
  (bind (_direction _move_track) (`Timeline|Move Object T`)
    (:`Update`
      (`self.K2_SetActorTransform` (`KismetMathLibrary.MakeTransform` (`SplineComponent.GetLocationAtDistanceAlongSpline` _spline (`KismetMathLibrary.Lerp` 0.0 (`SplineComponent.GetSplineLength` _spline) _move_track) "World") (`KismetMathLibrary.Conv_VectorToRotator` (`KismetMathLibrary.BreakRotIntoAxes` (`KismetMathLibrary.FindLookAtRotation` (`self.K2_GetActorLocation`) (`self.K2_GetActorLocation` (`GameplayStatics.GetPlayerPawn` 0))))))))))

(event `KillMe`
  (`self.K2_DestroyActor`))

(event `/Game/Characters/NPC/Enemies/I_Enemy.TakeDamage`
  (params (BaseDamage :type "Float (double-precision)") (DamageMultiplier :type "Float (double-precision)"))
  (bind _result (`/Engine/EditorBlueprintResources/StandardMacros.DecrementInt` (`self.HP`))
    (:`  `
      (if (<= _result 0)
        ;[1 1 1] Guardie dead code
        (`self.K2_DestroyActor` (`self.SplineRef`))
        (`self.K2_DestroyActor`)))))

(fn `FireSingle`
  (params (Source :type "StaticMeshComponent Object Reference"))
  (`|SpawnActorFromClass` "/Game/Weapons/BP_GuardieLaser.BP_GuardieLaser_C" (`SceneComponent.K2_GetComponentToWorld` Source) "Undefined" "MultiplyWithRoot" null (`GameplayStatics.GetPlayerController` 0) 0.0 0.0 null) ; Center
)

(fn `UserConstructionScript`)