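; Stickler turret enemy that aims its top ahead of the player and fires bursts of Guardie lasers.
; Tick sets the aim using the player's forward vector and max speed as lead, while overlap flags gate a delayed three-shot loop.
; Damage drains HP until it is destroyed, Bully and Wise Guy hits kill it outright, and lock-on toggles an overlay material.
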(event `self.ReceiveBeginPlay`
  (bind _asplayer_bp (cast `/Game/Characters/Player/PlayerBP` (`GameplayStatics.GetPlayerPawn` 0)))
  (set `self.Player` _asplayer_bp))

(event `self.ReceiveTick`
  (params (DeltaSeconds :type "Float (single-precision)"))
  (bind _player (`self.Player`))
  (`SceneComponent.K2_SetWorldRotation` (`self.SticklerTop`) (`KismetMathLibrary.Conv_VectorToRotator` (`KismetMathLibrary.BreakRotIntoAxes` (`KismetMathLibrary.FindLookAtRotation` (`self.K2_GetActorLocation`) (+ (`self.K2_GetActorLocation` _player) (* (`self.GetActorForwardVector` _player) (* (`MovementComponent.GetMaxSpeed` (`Character.CharacterMovement` _player)) (`self.PlayerOffset`))))))) false false)
  (if (`self.ShootTime`)
    (if (`self.SEMSeen`)
      (set `self.ShootTime` false)
      (`self.SEM Seen_Event`))))

(event `SEM Seen_Event`
  (bind _attack_delay (`self.Attack Delay`))
  (bind _returnvalue (`SceneComponent.K2_GetComponentToWorld` (`self.Cube`)))
  (bind _returnvalue_2 (/ _attack_delay 3.0))
  (`self.Shoot` _returnvalue)
  (`KismetSystemLibrary.Delay` _returnvalue_2)
  (`self.Shoot` _returnvalue)
  (`KismetSystemLibrary.Delay` _returnvalue_2)
  (`self.Shoot` _returnvalue)
  (`KismetSystemLibrary.Delay` _attack_delay) ; Wait a bit
  (set `self.ShootTime` true) ; Disconnected to match GDD
)

(event `self.ReceiveActorBeginOverlap`
  (params (OtherActor :type "Actor Object Reference"))
  (if (== (`GameplayStatics.GetObjectClass` OtherActor) "/Game/Characters/Player/PlayerBP.PlayerBP_C")
    (set `self.SEMSeen` true)))

(event `self.ReceiveActorEndOverlap`
  (params (OtherActor :type "Actor Object Reference"))
  (if (== (`GameplayStatics.GetObjectClass` OtherActor) "/Game/Characters/Player/PlayerBP.PlayerBP_C")
    (set `self.SEMSeen` false)))

(event `KillMe`
  (`self.K2_DestroyActor`))

(event `/Game/Characters/NPC/Enemies/I_Enemy.TakeDamage`
  (params (BaseDamage :type "Float (double-precision)") (ImpactLocation :type "Vector Structure"))
  (bind _output_get (set `self.HP` (- (`self.HP`) BaseDamage)))
  (if (<= _output_get 0.0)
    (`self.KillMe`)))

(event `/Game/Characters/NPC/Enemies/I_Enemy.DisplayLock`
  (`MeshComponent.SetOverlayMaterial` (`self.SticklerTop`) "/Game/Characters/NPC/M_LockOnOverlay.M_LockOnOverlay")
  (`MeshComponent.SetOverlayMaterial` (`self.SticklerBottom`) "/Game/Characters/NPC/M_LockOnOverlay.M_LockOnOverlay"))

(event `/Game/Characters/NPC/Enemies/I_Enemy.DisableLock`
  (`MeshComponent.SetOverlayMaterial` (`self.SticklerTop`) null)
  (`MeshComponent.SetOverlayMaterial` (`self.SticklerBottom`) null))

(fn `Damaged By Bully`
  (returns (`Enemy Destroyed` :type Boolean))
  (`self.KillMe`)
  (return true))

(fn `Damaged by Wise Guy`
  (returns (`Enemy Destroyed?` :type Boolean) (`Obstacle Destroyed?` :type Boolean))
  (`self.KillMe`)
  (return true false))

(fn `HitByProjectile`)

(fn `Shoot`
  (params (Target :type "Transform Structure"))
  (`|SpawnActorFromClass` "/Game/Weapons/BP_GuardieLaser.BP_GuardieLaser_C" (`KismetMathLibrary.MakeTransform` (.location Target) (.rotation Target)) "Undefined" "MultiplyWithRoot" null (`GameplayStatics.GetPlayerController` 0) 0.0 0.0 null) ; Center
)

(fn `UserConstructionScript`)