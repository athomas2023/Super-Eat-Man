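; GrubbrGuy boss spline Blueprint that calls StartBoss on BeginPlay, with no spline or movement logic of its own in this file.
; A CheckDistance event sketches rubber banding, marked as not working and not called here.
; It compares the boss Actor's X gap to the player against OptimalXDistance, then raises or lowers TimelineLength, with a minimum on decreases and debug prints.
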(event `self.ReceiveBeginPlay`
  (`parent.ReceiveBeginPlay`)
  (`self.StartBoss`))

(event `self.ReceiveTick`
  (params (DeltaSeconds :type "Float (single-precision)"))
  (`parent.ReceiveTick` DeltaSeconds))

(event `Check Distance`
  (bind _optimalxdistance (`self.OptimalXDistance`))
  (bind _timelinelength (`self.TimelineLength`))
  (bind _returnvalue_x (`KismetMathLibrary.BreakVector` (`self.K2_GetActorLocation` (`GameplayStatics.GetPlayerCharacter` 0))))
  (bind _returnvalue_x_2 (`KismetMathLibrary.BreakVector` (`self.K2_GetActorLocation` (`self.Actor`))))
  (bind _returnvalue (- _returnvalue_x_2 _returnvalue_x))
  ;[1 1 1] Rubber Banding, doesn't work
  (`KismetSystemLibrary.PrintString` (`KismetStringLibrary.Conv_DoubleToString` _returnvalue))
  (if (> _returnvalue _optimalxdistance)
    (set `self.TimelineLength` (+ (`self.TimelineLength`) 25.0))
    (elif (< _returnvalue _optimalxdistance)
      (set `self.TimelineLength` (`KismetMathLibrary.FMax` (- _timelinelength 25.0) 10.0))
      (`KismetSystemLibrary.PrintString` (`KismetStringLibrary.Conv_DoubleToString` _timelinelength)))))

(fn `UserConstructionScript`
  (`parent.UserConstructionScript`))