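; BP_GGPulseAttack is GrubbrGuy's pulse attack, an expanding ring that damages the player and expires after a fixed lifespan.
; Each tick grows OuterSphere uniformly and ZofAttack only in X and Y, keeping its height scale fixed.
; A hit requires the player to overlap both of those volumes but not InnerSphere, forming a height-limited hollow band.
; DoOnce limits each pulse to one SEMDamaged call on PlayerBP.
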(event `self.ReceiveBeginPlay`
  (set `self.Player` (`GameplayStatics.GetPlayerCharacter` 0))
  (`self.SetLifeSpan` 15.0))

(event `self.ReceiveTick`
  (params (DeltaSeconds :type "Float (single-precision)"))
  (bind _outersphere (`self.OuterSphere`))
  (bind _zofattack (`self.ZofAttack`))
  (bind _player (`self.Player`))
  (bind _scaletick (`self.ScaleTick`))
  (bind _scaletick_2 (`self.ScaleTick`))
  (`SceneComponent.SetWorldScale3D` _outersphere (`KismetMathLibrary.MakeVector` (+ (.x (`SceneComponent.K2_GetComponentScale` _outersphere)) _scaletick_2) (+ (.y (`SceneComponent.K2_GetComponentScale` _outersphere)) _scaletick_2) (+ (.z (`SceneComponent.K2_GetComponentScale` _outersphere)) _scaletick_2)))
  (`SceneComponent.SetWorldScale3D` _zofattack (`KismetMathLibrary.MakeVector` (+ (.x (`SceneComponent.K2_GetComponentScale` _zofattack)) _scaletick) (+ (.y (`SceneComponent.K2_GetComponentScale` _zofattack)) _scaletick) (.z (`SceneComponent.K2_GetComponentScale` _zofattack))))
  (if (`PrimitiveComponent.IsOverlappingActor` (`self.InnerSphere`) _player)
    _
    (elif (`PrimitiveComponent.IsOverlappingActor` (`self.ZofAttack`) _player)
      (if (`PrimitiveComponent.IsOverlappingActor` (`self.OuterSphere`) _player)
        (`/Engine/EditorBlueprintResources/StandardMacros.DoOnce` false
          (:`Completed`
            (bind _asplayer_bp (cast `/Game/Characters/Player/PlayerBP` (`GameplayStatics.GetPlayerPawn` 0)))
            (`/Game/Characters/Player/PlayerBP.SEM Damaged` _asplayer_bp)))))))

(fn `UserConstructionScript`)