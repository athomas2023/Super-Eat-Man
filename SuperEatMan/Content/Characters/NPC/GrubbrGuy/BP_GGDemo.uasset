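; GrubbrGuy (GG) demo NPC that attacks the player, shows health as text and is destroyed at zero.
; BeginPlay starts a recursive bomb-spawning loop and a looping timer that randomly toggles spinning.
; Movement events run a Timeline along runtime-built splines for random paths, arced jumps and slam descents, using splines because physics conflicted with movement.
; Pulse and projectile attacks, physics Jump and debug damage are defined but not called here.
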(event `self.ReceiveBeginPlay`
  (set `self.Health` (`self.MaxHealth`))
  (`self.DisplayHealth`) ; Update GG's Health Display to Current
  (`KismetSystemLibrary.K2_SetTimerDelegate` (delegate `SpinCheck`) (`self.SpinTimer`) true) ; Sets that every "spin timer" seconds, the spin check event is called
  (`self.Shoot` 0.1))

(event `PlaceSpline`
  (`self.Generate Spline`))

(event `self.ReceiveTick`
  (params (DeltaSeconds :type "Float (single-precision)")))

(event `StopMoving`
  (bind _myspline (`self.MySpline`))
  ;[1 1 1] Move On Spline (Should be called each tick GG is moving along spline)
  (bind (_direction _move_track) (`Timeline|Timeline` :!via `Stop` :!label _label)
    (:`Update`
      (bind _returnvalue (`SplineComponent.GetLocationAtDistanceAlongSpline` _myspline (`KismetMathLibrary.Lerp` 0.0 (`SplineComponent.GetSplineLength` _myspline) _move_track) "World"))
      (`SceneComponent.K2_SetWorldLocation` (`self.GGRoot`) _returnvalue false false)
      (if (`self.IsJumping`)
        (if (< (`KismetMathLibrary.Abs` (`KismetMathLibrary.VSize` (- _returnvalue (`SplineComponent.GetLocationAtSplinePoint` (`self.MySpline`) 1 "World")))) 10.0)
          (set `self.SlamAttack` true)))
      (set `self.IsMoving` true))
    (:`Finished`
      (`ActorComponent.K2_DestroyComponent` (`self.MySpline`))
      (set `self.IsMoving` false)
      (set `self.CanMove` false)
      (set `self.IsJumping` false))))

(event `MoveAlongSpline`
  (params (Speed :type "Float (double-precision)" :default 5.0))
  (bind _timeline (`self.Timeline`))
  ;[1 1 1] Move On Spline (Should be called each tick GG is moving along spline)
  (if (`self.CanMove`)
    (if (`self.IsJumping`)
      (`TimelineComponent.SetPlayRate` _timeline 1.0)
      (else
        (`TimelineComponent.SetPlayRate` _timeline (/ 1.0 Speed))))
    (if (`self.IsMoving`)
      (goto _label)
      (else
        (goto _label :!via `PlayFromStart`)))))

(event `Shoot`
  (params (ShootDelay :type "Float (double-precision)"))
  ;[1 1 1] Shoot projectile from left and right source. RECURSIVE FOR TESTING
  (`self.Bomb` :!label _label_2)
  (`KismetSystemLibrary.Delay` ShootDelay :!label _label_3)
  (if (`self.CanShoot`)
    (goto _label_2)
    (else
      (goto _label_3))))

(event `/Game/Characters/NPC/Enemies/I_Enemy.TakeDamage`
  (`self.DamageGG`))

(event `SlamDown`
  (set `self.IsMoving` false)
  (set `self.CanMove` false)
  (set `self.IsJumping` false)
  (`self.DownSpline`)
  (`KismetSystemLibrary.Delay` (`KismetMathLibrary.RandomFloatInRange` 0.02 1.0))
  (`self.MoveAlongSpline` 5.0))

(event `Ouch`
  ;[0.05185 1 0.4373] For Debugging Health! Recursive Function ONLY CALL ONCE
  (`KismetSystemLibrary.Delay` 2.5)
  (`/Game/Characters/NPC/Enemies/I_Enemy.TakeDamage`)
  (`self.Ouch`))

(event `Spin`
  ;[1 1 1] The Spinning Code
  (if (not (`self.IsSpinning`))
    (set `self.IsSpinning` true)
    (if (`self.IsSpinning`)
      (if (`self.CanSpin`) :!label _label_4
        (`SceneComponent.K2_AddLocalRotation` (`self.GGRoot`) (`KismetMathLibrary.MakeRotator` 0.0 0.0 (* (`GameplayStatics.GetWorldDeltaSeconds`) (`self.SpinSpeed`))) false false)
        (`KismetSystemLibrary.DelayUntilNextTick`)
        (goto _label_4)
        (else
          (`self.StopSpin`))))))

(event `StopSpin`
  ;[1 1 1] The Spinning Code
  (set `self.IsSpinning` false)
  (`SceneComponent.K2_SetWorldRotation` :`self` (`self.GGRoot`)))

(event `SpinCheck`
  ;[1 1 1] The Spinning Code
  (if (`self.CanSpin`)
    (if (`self.IsSpinning`)
      (if (`self.IsJumping`)
        _
        (else
          _))
      ;;[1 1 1] Chance of stopping spinning
      (if (< (`KismetMathLibrary.RandomInteger` 100) (`self.StopSpinChance`))
        (`self.StopSpin`))
      (else
        ;;[1 1 1] Chance of starting spinning
        (if (< (`KismetMathLibrary.RandomInteger` 100) (`self.SpinChance`))
          (`self.Spin`))))))

(fn `Bomb`
  (bind _returnvalue (`|SpawnActorFromClass` "/Game/Weapons/BP_GGBomb.BP_GGBomb_C" (`SceneComponent.K2_GetComponentToWorld` (`self.GGRoot`)) "Undefined" "MultiplyWithRoot" null (`GameplayStatics.GetPlayerCharacter` 0) 1.0 0.0 null))
  (`self.K2_AttachToActor` _returnvalue self "None" "KeepWorld" "KeepWorld" "KeepWorld" true))

(fn `DamageGG`
  (bind _output_get (set `self.Health` (- (`self.Health`) 1)))
  (`self.DisplayHealth`) ; Update Health Displayed by GG
  (if (<= _output_get 0)
    (`self.K2_DestroyActor`)))

(fn `DisplayHealth`
  (`TextRenderComponent.K2_SetText` (`self.TextRender`) (`KismetTextLibrary.Conv_StringToText` (`KismetStringLibrary.Concat_StrStr` (`KismetStringLibrary.Concat_StrStr` (`KismetStringLibrary.Conv_IntToString` (`self.Health`)) "/") (`KismetStringLibrary.Conv_IntToString` (`self.MaxHealth`))))))

(fn `DownSpline`
  (bind _ggroot (`self.GGRoot`))
  (bind _myspline (`self.MySpline`))
  (bind _returnvalue (`SceneComponent.K2_GetComponentLocation` _ggroot))
  ;[1 1 1] GG will generate the spline for going down
  (if (not (== (`self.MySpline`) null))
    (`ActorComponent.K2_DestroyComponent` (`self.MySpline`)))
  (bind _returnvalue_2 (`AddComponent|NODE_AddSplineComponent-2` :`RelativeTransform` (`SceneComponent.GetRelativeTransform` _ggroot)))
  (set `self.MySpline` _returnvalue_2)
  (`SplineComponent.SetLocationAtSplinePoint` _myspline 0 _returnvalue "World" true) ; Point at GG's current location
  (`SplineComponent.SetLocationAtSplinePoint` _myspline 1 (`KismetMathLibrary.MakeVector` (.x _returnvalue) (.y _returnvalue) (.z (`SceneComponent.K2_GetComponentLocation` (`self.The ground`)))) "World" true) ; Ground
  (set `self.CanMove` true)
  (return))

(fn `FollowSpline`
  (`TimelineComponent.SetPlayRate` (`self.Timeline`) (/ 1.0 (`self.TimeToComplete`)))
  (if true
    _))

(fn `Generate Spline`
  (locals (BoxMultiplier :type "Float (double-precision)" :default 8.0))
  (bind _ggroot (`self.GGRoot`))
  (bind _myspline (`self.MySpline`))
  (bind _returnvalue (`SplineComponent.GetNumberOfSplinePoints` (`self.MySpline`)))
  (if (not (== (`self.MySpline`) null))
    (`ActorComponent.K2_DestroyComponent` (`self.MySpline`)))
  ;[1 1 1] Make a new spline
  (bind _returnvalue_2 (`AddComponent|NODE_AddSplineComponent-0` :`RelativeTransform` (`SceneComponent.GetRelativeTransform` _ggroot)))
  (set `self.MySpline` _returnvalue_2)
  (`SplineComponent.SetLocationAtSplinePoint` _myspline 0 (`KismetMathLibrary.MakeVector` (.x (`SceneComponent.K2_GetComponentLocation` _ggroot)) (.y (`SceneComponent.K2_GetComponentLocation` _ggroot)) (.z (`SceneComponent.K2_GetComponentLocation` (`self.Bounds`)))) "World" true)
  (`SplineComponent.SetLocationAtSplinePoint` _myspline 1 (`self.RandomLocInBounds`) "World" true)
  (for _index (range _returnvalue 11)
    (`KismetSystemLibrary.PrintString` (`KismetStringLibrary.Conv_IntToString` _returnvalue))
    (`self.SplineMagic` _index))
  (set `self.CanMove` true)
  (return))

(fn `Jump`
  (returns (JumpComplete :type Boolean))
  (locals (DistanceWindow :type "Float (double-precision)" :default 1e-06) (JumpArc :type "Float (single-precision)" :default 0.1))
  (bind _ggroot (`self.GGRoot`))
  (if (not (`self.IsJumping`))
    (set `self.IsJumping` true)
    (bind _output_get (set `self.JumpTarget` (`self.RandomLocInBounds`)))
    ;[1 1 1] OLD
    (bind _outlaunchvelocity (`GameplayStatics.SuggestProjectileVelocity_CustomArc` (`SceneComponent.K2_GetComponentLocation` (`self.GGRoot`)) _output_get 0.0 (`local.JumpArc`)))
    (bind _output_get_2 (set `self.GGVelocity` (* _outlaunchvelocity (`KismetMathLibrary.Conv_DoubleToVector` 100.0))))
    (`PrimitiveComponent.AddImpulseAtLocation` _ggroot _output_get_2 (`SceneComponent.K2_GetComponentLocation` _ggroot) "None")
    (return false)))

(fn `PulseAttack`
  (returns (Pulse :type "/Game/Characters/NPC/GrubbrGuy/BP_GGPulseAttack Object Reference"))
  (bind _returnvalue (`SceneComponent.K2_GetComponentToWorld` (`self.GGRoot`)))
  (bind _returnvalue_2 (`|SpawnActorFromClass` "/Game/Characters/NPC/GrubbrGuy/BP_GGPulseAttack.BP_GGPulseAttack_C" (`KismetMathLibrary.MakeTransform` (`KismetMathLibrary.MakeVector` (.x (.location _returnvalue)) (.y (.location _returnvalue)) (.z (.location (`SceneComponent.K2_GetComponentToWorld` (`self.The ground`)))))) "Undefined" "MultiplyWithRoot" null null))
  (`self.K2_AttachToActor` _returnvalue_2 self "None" "KeepWorld" "KeepWorld" "KeepWorld" true)
  (return _returnvalue_2))

(fn `ShootProjectile`
  (params (Source :type "Transform Structure"))
  (`|SpawnActorFromClass` "/Game/Weapons/BP_GGProjectile.BP_GGProjectile_C" (`KismetMathLibrary.MakeTransform` (.location Source) (.rotation Source)) "Undefined" "MultiplyWithRoot" null (`GameplayStatics.GetPlayerController` 0) 0.0 0.0 null) ; Center
)

(fn `SplineArc`
  (locals (MinJumpHeight :type "Float (double-precision)" :default 100.0) (MaxJumpHeight :type "Float (double-precision)" :default 300.0) (JumpStart :type "Vector Structure") (JumpEnd :type "Vector Structure"))
  (bind _ggroot (`self.GGRoot`))
  (bind _myspline (`self.MySpline`))
  ;[1 1 1] Spline is used instead of physics, as physics wasn't playing nice with the movement code
  (if (not (== (`self.MySpline`) null))
    (`ActorComponent.K2_DestroyComponent` (`self.MySpline`)))
  (bind _returnvalue (`AddComponent|NODE_AddSplineComponent-1` :`RelativeTransform` (`SceneComponent.GetRelativeTransform` _ggroot)))
  (set `self.MySpline` _returnvalue)
  (bind _output_get (set `local.JumpStart` (`SceneComponent.K2_GetComponentLocation` _ggroot)))
  (`SplineComponent.SetLocationAtSplinePoint` _myspline 0 _output_get "World" true) ; Point at GG's current location
  (bind _output_get_2 (set `local.JumpEnd` (`self.RandomLocInBounds`)))
  (`SplineComponent.SetLocationAtSplinePoint` _myspline 1 (`KismetMathLibrary.MakeVector` (/ (+ (.x (`local.JumpStart`)) (.x (`local.JumpEnd`))) 2.0) (/ (+ (.y (`local.JumpStart`)) (.y (`local.JumpEnd`))) 2.0) (+ (.z (`local.JumpEnd`)) (`KismetMathLibrary.RandomFloatInRange` (`local.MinJumpHeight`) (`local.MaxJumpHeight`)))) "World" true) ; Top of Jump
  (`SplineComponent.AddSplinePointAtIndex` (`self.MySpline`) _output_get_2 2 "World" true) ; End of Jump
  (set `self.CanMove` true)
  (set `self.IsJumping` true)
  (return))

(fn `SplineMagic`
  (params (SplineIndex :type Integer))
  (`SplineComponent.AddSplinePointAtIndex` (`self.MySpline`) (`self.RandomLocInBounds`) SplineIndex "World" true))

(fn `UserConstructionScript`)