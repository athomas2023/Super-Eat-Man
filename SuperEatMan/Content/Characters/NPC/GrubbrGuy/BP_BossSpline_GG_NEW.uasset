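; Boss spline actor for the GrubbrGuy NPC, in a mostly stubbed state.
; BeginPlay casts the player character to PlayerBP and caches the reference.
; Unreachable leftover logic would start the boss, destroy the Box component and call StartUp on a BP_GGDemo actor.
; Tick is empty, the parent BeginPlay call is disabled, and the construction script only calls its parent.
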(event `self.ReceiveBeginPlay`
  (bind _asplayer_bp (cast `/Game/Characters/Player/PlayerBP` (`GameplayStatics.GetPlayerCharacter` 0)))
  (set `self.PlayerBPRef` _asplayer_bp))

(fn `UserConstructionScript`
  (`parent.UserConstructionScript`))