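; AI controller for the saucer NPC, with helpers for sighting the player and shooting.
; HandleSightSense stores the sighted player in the TargetActor blackboard key and returns sight state.
; Fire aims the saucer mesh at the player and spawns a drone projectile, though nothing here calls either function.
; Event graph logic for possession, BT_Globber, laser bursts and looped turning is disconnected, so it never runs.
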(event `self.ReceivePossess`
  (params (PossessedPawn :type "Pawn Object Reference"))
  ;[0.8906 0.03542 0.008838] Comment
)

(event `self.ReceiveBeginPlay`)

(event `Face Player`)

(fn `Fire`
  (bind _mesh (`Character.Mesh` (`self.BP Saucer Ref`)))
  ;[1 1 1] Shooting
  (`SceneComponent.K2_SetWorldRotation` _mesh (`KismetMathLibrary.FindLookAtRotation` (`SceneComponent.K2_GetComponentLocation` _mesh) (`SceneComponent.K2_GetComponentLocation` (`Character.Mesh` (`GameplayStatics.GetPlayerCharacter` 0)))) false false)
  (`|SpawnActorFromClass` "/Game/Weapons/DroneProjectile_BP.DroneProjectile_BP_C" (`SceneComponent.K2_GetComponentToWorld` (`Character.Mesh` (`self.BP Saucer Ref`))) "Undefined" "MultiplyWithRoot" null null null))

(fn `HandleSightSense`
  (params (Actor :type "Actor Object Reference") (Stimulus :type "AIStimulus Structure"))
  (returns (`In Sight` :type Boolean) (`Targeted Actor` :type "Actor Object Reference"))
  (bind (_stimulus_age _stimulus_expirationage _stimulus_strength _stimulus_stimuluslocation _stimulus_receiverlocation _stimulus_tag _stimulus_bsuccessfullysensed) (break `AIStimulus` (`local.Stimulus`)))
  (bind _returnvalue (`AIPerceptionSystem.GetSenseClassForStimulus` Stimulus))
  (if (== _returnvalue "/Script/AIModule.AISense_Sight")
    (if (== (`local.Actor`) (`GameplayStatics.GetPlayerCharacter` 0))
      (`BlackboardComponent.SetValueAsObject` (`self.Blackboard`) "TargetActor" (`local.Actor`))
      (return _stimulus_bsuccessfullysensed (`local.Actor`)))))

(fn `UserConstructionScript`)