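; Saucer NPC enemy that fires a red laser at a target actor and dies when its health runs out.
; ActivateLaserBurst line-traces to the target, feeding the hit point to Niagara beam and impact effects, shown only on a blocking hit.
; The trace starts at a normalized forward vector, without the saucer's location added.
; DamageTaken decrements and prints health, then at zero destroys the actor and calls GlobberKilled.
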(event `self.ReceiveBeginPlay`
  (`SceneComponent.SetVisibility` (`self.Niagara Laser`) false false)
  (`SceneComponent.SetVisibility` (`self.Niagara Laser Impact`) false false)
  (`FXSystemComponent.SetColorParameter` (`self.Niagara Laser`) "Color" (struct :`R` 1.0 :`B` 0.029524 :`A` 1.0))
  (`FXSystemComponent.SetColorParameter` (`self.Niagara Laser Impact`) "Color" (struct :`R` 1.0 :`B` 0.029524 :`A` 1.0)))

(event `Activate Laser Burst`
  (params (`Target Actor` :type "Actor Object Reference"))
  (bind _output_get (set `self.Target Actor` `Target Actor`))
  (`/Engine/EditorBlueprintResources/StandardMacros.IsValid` _output_get
    (:`Is Valid`
      (bind _output_get_2 (set `self.Trace End` (`self.K2_GetActorLocation` (`self.Target Actor`))))
      (bind _outhit (`KismetSystemLibrary.LineTraceSingle` (`KismetMathLibrary.Normal` (* (`self.GetActorForwardVector`) 800.0)) _output_get_2 "TraceTypeQuery3"))
      (set `self.Blocked Hit` (`GameplayStatics.BreakHitResult` _outhit))
      (set `self.Hit Location` (`.Location` (`GameplayStatics.BreakHitResult` _outhit)))
      (`SceneComponent.SetVisibility` (`self.Niagara Laser`) (`self.Blocked Hit`) false)
      (`FXSystemComponent.SetVectorParameter` (`self.Niagara Laser`) "LaserEnd" (`self.Hit Location`))
      (`FXSystemComponent.SetVectorParameter` (`self.Niagara Laser Impact`) "ImpactLocation" (`self.Hit Location`))
      (`SceneComponent.SetVisibility` (`self.Niagara Laser Impact`) (`self.Blocked Hit`) false))))

(event `Deactivate Laser Burst`
  (`SceneComponent.SetVisibility` (`self.Niagara Laser`) false false)
  (`SceneComponent.SetVisibility` (`self.Niagara Laser Impact`) false false))

(event `Damage Taken`
  ;[1 1 1] Death
  (bind _result (`/Engine/EditorBlueprintResources/StandardMacros.DecrementInt` (`self.Enemy Health`))
    (:`  `
      (`KismetSystemLibrary.PrintString` (`KismetStringLibrary.Concat_StrStr` "Enemy Health:  " (`KismetStringLibrary.Conv_IntToString` _result)))
      (if (<= _result 0)
        (`self.K2_DestroyActor`)
        (`self.GlobberKilled`)))))

(fn `UserConstructionScript`)