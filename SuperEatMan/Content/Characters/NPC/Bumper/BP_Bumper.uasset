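; BP_Bumper is a robot NPC that acts as a proximity bomb against the player and can be destroyed by damage.
; The player entering its sphere triggers a one-time beep warning and a timer, after which it plays an explosion sound, applies full radial damage and destroys itself.
; Incoming damage plays sound and spark effects and lowers health; at zero it spawns an explosion effect and is destroyed without applying radial damage.
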(event `self.ReceiveBeginPlay`
  (bind _asplayer_bp (cast `/Game/Characters/Player/PlayerBP` (`GameplayStatics.GetPlayerCharacter` 0)))
  (set `self.PlayerBP Ref` _asplayer_bp))

(event `self.Sphere.OnComponentBeginOverlap`
  (params (OverlappedComponent :type "PrimitiveComponent Object Reference") (OtherActor :type "Actor Object Reference") (OtherComp :type "PrimitiveComponent Object Reference") (OtherBodyIndex :type Integer) (bFromSweep :type Boolean) (SweepResult :type "HitResult Structure (by ref)"))
  (cast `/Game/Characters/Player/PlayerBP` OtherActor)
  (`/Engine/EditorBlueprintResources/StandardMacros.DoOnce` false
    (:`Completed`
      (`GameplayStatics.PlaySound2D` "/Game/Sound/SFX/beep.beep" 1.0 1.0 0.0 null null)
      (`KismetSystemLibrary.Delay` 0.3)
      (`GameplayStatics.PlaySound2D` "/Game/Sound/SFX/Longbeep.Longbeep" 1.0 1.0 0.0 null null)
      (`KismetSystemLibrary.K2_SetTimerDelegate` (delegate `Detonate`) 1.5))))

(event `Detonate`
  (bind _returnvalue_location (`KismetMathLibrary.BreakTransform` (`self.GetTransform`)))
  (`GameplayStatics.PlaySound2D` "/Game/Sound/SFX/explosion.explosion" 1.0 1.0 0.0 null null)
  (`GameplayStatics.ApplyRadialDamage` :`BaseDamage` 0.5 :`Origin` _returnvalue_location :`DamageRadius` 2500.0 :`DamageCauser` self :`InstigatedByController` null :`bDoFullDamage` true)
  (`self.K2_DestroyActor`))

(event `/Game/Characters/NPC/Enemies/I_Enemy.TakeDamage`
  (params (BaseDamage :type "Float (double-precision)") (ImpactLocation :type "Vector Structure"))
  (`GameplayStatics.PlaySoundAtLocation` "/Game/Sound/SFX/RobotDamaged.RobotDamaged" (`SceneComponent.K2_GetComponentLocation` (`self.SkeletalMesh`)) (struct) 1.0 1.0 0.0 null null null null)
  (`NiagaraFunctionLibrary.SpawnSystemAtLocation` "/Game/Effects/VFX/NS/DamageSpark_NS.DamageSpark_NS" (`SceneComponent.K2_GetComponentLocation` (`self.SkeletalMesh`)) (struct :`Roll` 90.0) (0.01 0.01 0.01))
  (bind _output_get (set `self.Health` (- (`self.Health`) BaseDamage)))
  (if (<= _output_get 0.0)
    (`NiagaraFunctionLibrary.SpawnSystemAtLocation` "/Game/Effects/VFX/NS/Explod.Explod" (`SceneComponent.K2_GetComponentLocation` (`self.SkeletalMesh`)) (struct :`Roll` 90.0))
    (`self.K2_DestroyActor`)))

(fn `UserConstructionScript`)