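; BP_Jiffy is a robot NPC that moves along a spline and damages the player with two saws.
; On BeginPlay a timeline, its play rate scaled by TimeToComplete, drives the body's position along the spline and animates its pitch.
; Overlapping either saw calls SEMDamaged on PlayerBP.
; TakeDamage plays a sound and sparks, decrements Health, and at zero spawns an explosion and destroys the actor.
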(event `self.ReceiveBeginPlay`
  ;[1 1 1] Start Movement
  (`self.Move Along Spline`))

(event `Move Along Spline`
  ;[1 1 1] Movement Alone Spline
  (`TimelineComponent.SetPlayRate` (`self.Jiffy Timeline`) (/ 1.0 (`self.Time to Complete`)))
  (bind (_direction _movement_track _tilt_track) (`Timeline|Jiffy Timeline` :!via `PlayFromStart`) ; Ensure Length is Set to 1 - else play rate will not work as intended
    (:`Update`
      (bind _returnvalue_location (`KismetMathLibrary.BreakTransform` (`SplineComponent.GetTransformAtDistanceAlongSpline` (`self.Spline`) (`KismetMathLibrary.Lerp` 0.0 (`SplineComponent.GetSplineLength` (`self.Spline`)) _movement_track) "Local" false)))
      (`SceneComponent.K2_SetRelativeTransform` (`self.Jiffy Body`) (`KismetMathLibrary.MakeTransform` _returnvalue_location (struct) (2.0 2.0 2.0)) false false)
      (`SceneComponent.K2_SetRelativeRotation` (`self.Jiffy Body`) (`KismetMathLibrary.MakeRotator` 180.0 _tilt_track 180.0) false false))))

(event `self.Right Saw.OnComponentBeginOverlap`
  (params (OverlappedComponent :type "PrimitiveComponent Object Reference") (OtherActor :type "Actor Object Reference") (OtherComp :type "PrimitiveComponent Object Reference") (OtherBodyIndex :type Integer) (bFromSweep :type Boolean) (SweepResult :type "HitResult Structure (by ref)"))
  ;[1 1 1] Kill SEM
  (bind _asplayer_bp (cast `/Game/Characters/Player/PlayerBP` OtherActor))
  (`/Game/Characters/Player/PlayerBP.SEM Damaged` _asplayer_bp))

(event `self.Left Saw.OnComponentBeginOverlap`
  (params (OverlappedComponent :type "PrimitiveComponent Object Reference") (OtherActor :type "Actor Object Reference") (OtherComp :type "PrimitiveComponent Object Reference") (OtherBodyIndex :type Integer) (bFromSweep :type Boolean) (SweepResult :type "HitResult Structure (by ref)"))
  ;[1 1 1] Kill SEM
  (bind _asplayer_bp (cast `/Game/Characters/Player/PlayerBP` OtherActor))
  (`/Game/Characters/Player/PlayerBP.SEM Damaged` _asplayer_bp))

(event `/Game/Characters/NPC/Enemies/I_Enemy.TakeDamage`
  (params (BaseDamage :type "Float (double-precision)") (ImpactLocation :type "Vector Structure"))
  (`GameplayStatics.PlaySoundAtLocation` "/Game/Sound/SFX/RobotDamaged.RobotDamaged" (`SceneComponent.K2_GetComponentLocation` (`self.Jiffy Body`)) (struct) 1.0 1.0 0.0 null null null null)
  (`NiagaraFunctionLibrary.SpawnSystemAtLocation` "/Game/Effects/VFX/NS/DamageSpark_NS.DamageSpark_NS" (`SceneComponent.K2_GetComponentLocation` (`self.Jiffy Body`)) (struct :`Roll` 90.0) (0.01 0.01 0.01))
  (bind _result (`/Engine/EditorBlueprintResources/StandardMacros.DecrementInt` (`self.Health`))
    (:`  `
      (if (<= _result 0)
        (`NiagaraFunctionLibrary.SpawnSystemAtLocation` "/Game/Effects/VFX/NS/Explod.Explod" (`SceneComponent.K2_GetComponentLocation` (`self.Jiffy Body`)) (struct :`Roll` 90.0))
        (`self.K2_DestroyActor`)))))

(fn `UserConstructionScript`)