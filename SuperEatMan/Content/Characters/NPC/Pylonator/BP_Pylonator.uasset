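; Pylonator boss NPC that starts its spline reference and a looping attack timer when a non-ragdolling player enters its detection area.
; Each attack randomly spawns either a sweep projectile or pillar projectiles at three distinct points out of four, all short-lived.
; StopBossAttack clears the timer and stops the spline timeline.
; Damage handlers flash an overlay, play sound and FX, and decrement HP, with death checked there and on Tick.
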(event `StopBossAttack`
  ;[1 1 1] Pylonator Shooting
  ;;[1 1 1] Stop Boss Attack
  (`KismetSystemLibrary.K2_ClearAndInvalidateTimerHandle` (stale `self.DetectionArea.OnComponentBeginOverlap` _returnvalue))
  (set `self.BossAttacking` false)
  (`/Game/Characters/NPC/Pylonator/BP_BossSpline.StopTimeline` (`self.BossSplineRef`)))

(event `self.DetectionArea.OnComponentBeginOverlap`
  (params (OverlappedComponent :type "PrimitiveComponent Object Reference") (OtherActor :type "Actor Object Reference") (OtherComp :type "PrimitiveComponent Object Reference") (OtherBodyIndex :type Integer) (bFromSweep :type Boolean) (SweepResult :type "HitResult Structure (by ref)"))
  ;[1 1 1] Pylonator Shooting
  (bind _asplayer_bp (cast `/Game/Characters/Player/PlayerBP` (`GameplayStatics.GetPlayerPawn` 0)))
  (if (and (== _asplayer_bp OtherActor) (not (`/Game/Characters/Player/PlayerBP.Ragdolling` _asplayer_bp)))
    (if (not (`self.BossAttacking`))
      (set `self.BossAttacking` true)
      (`/Game/Characters/NPC/Pylonator/BP_BossSpline.StartBoss` (`self.BossSplineRef`))
      (bind _returnvalue (`KismetSystemLibrary.K2_SetTimer` null "StartBossAttack" 2.0 true)))))

(event `Take Damage`
  ;[1 1 1] Pylonator Health
  (`MeshComponent.SetOverlayMaterial` (`self.PylonatorBody`) "/Game/Characters/NPC/M_DamageOverlay.M_DamageOverlay")
  (`KismetSystemLibrary.Delay` 0.3)
  (`MeshComponent.SetOverlayMaterial` (`self.PylonatorBody`) null)
  (`/Engine/EditorBlueprintResources/StandardMacros.DecrementInt` (`self.BossHP`)))

(event `Kill Pylonator`
  ;[1 1 1] Pylonator Health
  (`self.K2_DestroyActor`))

(event `self.ReceiveTick`
  (params (DeltaSeconds :type "Float (single-precision)"))
  ;[1 1 1] Pylonator Health
  (`|ExecutionSequence`
    (:`then_0`
      (if (<= (`self.BossHP`) 0)
        (`self.Kill Pylonator`)))))

(event `/Game/Characters/NPC/Enemies/I_Enemy.TakeDamage`
  (`MeshComponent.SetOverlayMaterial` (`self.PylonatorBody`) "/Game/Characters/NPC/M_DamageOverlay.M_DamageOverlay")
  (`KismetSystemLibrary.Delay` 0.3)
  (`MeshComponent.SetOverlayMaterial` (`self.PylonatorBody`) null)
  (`GameplayStatics.PlaySoundAtLocation` "/Game/Sound/SFX/RobotDamaged.RobotDamaged" (`SceneComponent.K2_GetComponentLocation` (`self.PylonatorBody`)) (struct) 1.0 1.0 0.0 null null null null)
  (`NiagaraFunctionLibrary.SpawnSystemAtLocation` "/Game/Weapons/FX_WiseGuy.FX_WiseGuy" (`SceneComponent.K2_GetComponentLocation` (`self.PylonatorBody`)) (struct :`Roll` 90.0) (0.01 0.01 0.01))
  (bind _result (`/Engine/EditorBlueprintResources/StandardMacros.DecrementInt` (`self.BossHP`))
    (:`  `
      (if (<= _result 0)
        (`self.K2_DestroyActor`)))))

(fn `GetRandomNumberList`
  (params (`Range Lower Bound` :type Integer) (`Range Upper Bound` :type Integer :default 3) (`Numbers Selected Count` :type Integer :default 3))
  (returns (SpawnLocations :type "Array of Integer"))
  (bind _spawnlocations (`self.SpawnLocations`))
  (`KismetArrayLibrary.Array_Clear` (`self.SpawnLocations`))
  (bind _output_get (set `self.Temporary Spawn Point` (`KismetMathLibrary.RandomIntegerInRange` `Range Lower Bound` `Range Upper Bound`) :!label _label))
  (if (`KismetArrayLibrary.Array_Contains` _spawnlocations _output_get) :!label _label_2
    (goto _label)
    (else
      (`KismetArrayLibrary.Array_Add` _spawnlocations _output_get)
      (if (< (`KismetArrayLibrary.Array_Length` _spawnlocations) (`local.Numbers Selected Count`))
        (goto _label_2)
        (else
          (return _spawnlocations))))))

(fn `StartBossAttack`
  (if (`self.BossAttacking`)
    (switch `int` (`KismetMathLibrary.RandomIntegerInRange` 0 1)
      (:`0`
        (bind _returnvalue (`|SpawnActorFromClass` "/Game/Weapons/BP_PylonatorProjectileSWEEP.BP_PylonatorProjectileSWEEP_C" (`SceneComponent.K2_GetComponentToWorld` (`self.SpawnPoint5`)) "Undefined" "MultiplyWithRoot" self null))
        (`self.SetLifeSpan` _returnvalue 6.0))
      (:`1`
        (bind _spawnlocations (`self.GetRandomNumberList` 0))
        (for _array_element _spawnlocations
          (switch `int` _array_element
            (:`0`
              (bind _returnvalue_2 (`|SpawnActorFromClass` "/Game/Weapons/BP_PylonatorProjectilePILLAR.BP_PylonatorProjectilePILLAR_C" (`SceneComponent.K2_GetComponentToWorld` (`self.SpawnPoint1`)) "Undefined" "MultiplyWithRoot" self null)))
            (:`1`
              (bind _returnvalue_3 (`|SpawnActorFromClass` "/Game/Weapons/BP_PylonatorProjectilePILLAR.BP_PylonatorProjectilePILLAR_C" (`SceneComponent.K2_GetComponentToWorld` (`self.SpawnPoint2`)) "Undefined" "MultiplyWithRoot" self null)))
            (:`2`
              (bind _returnvalue_4 (`|SpawnActorFromClass` "/Game/Weapons/BP_PylonatorProjectilePILLAR.BP_PylonatorProjectilePILLAR_C" (`SceneComponent.K2_GetComponentToWorld` (`self.SpawnPoint3`)) "Undefined" "MultiplyWithRoot" self null)))
            (:`3`
              (bind _returnvalue_5 (`|SpawnActorFromClass` "/Game/Weapons/BP_PylonatorProjectilePILLAR.BP_PylonatorProjectilePILLAR_C" (`SceneComponent.K2_GetComponentToWorld` (`self.SpawnPoint4`)) "Undefined" "MultiplyWithRoot" self null))))
          (`self.SetLifeSpan` _returnvalue_2 6.0)
          (`self.SetLifeSpan` _returnvalue_3 6.0)
          (`self.SetLifeSpan` _returnvalue_5 6.0)
          (`self.SetLifeSpan` _returnvalue_4 6.0))))))

(fn `UserConstructionScript`)