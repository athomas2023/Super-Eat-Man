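; BP_BossIntroTrigger is a trigger actor that plays a brief boss intro screen when the player enters its volume.
; On the first player overlap only, it disables player control and hides the HUD and mouse cursor.
; It switches on the level name to show the Foredrone, Pylonator or GrubberGuy intro widget.
; After a fixed delay, it removes the widget and restores control, HUD and cursor.
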(event `self.ReceiveBeginPlay`
  (bind _asplayer_bp (cast `/Game/Characters/Player/PlayerBP` (`GameplayStatics.GetPlayerCharacter` 0)))
  (set `self.As Player BP` _asplayer_bp))

(event `self.StartTrigger.OnComponentBeginOverlap`
  (params (OverlappedComponent :type "PrimitiveComponent Object Reference") (OtherActor :type "Actor Object Reference") (OtherComp :type "PrimitiveComponent Object Reference") (OtherBodyIndex :type Integer) (bFromSweep :type Boolean) (SweepResult :type "HitResult Structure (by ref)"))
  (bind _returnvalue (`GameplayStatics.GetPlayerController` 0))
  (bind _as_player_bp (`self.As Player BP`))
  (if (== OtherActor _as_player_bp)
    (`/Engine/EditorBlueprintResources/StandardMacros.DoOnce` false
      (:`Completed`
        (set `/Game/Characters/Player/PlayerBP.IsPlayerCotrollerEnabled?` false _as_player_bp)
        (bind _returnvalue_2 (`GameplayStatics.GetCurrentLevelName` true))
        (`Widget.SetVisibility` (`/Game/Characters/Player/PlayerBP.HeadsUpDisplayRef` (`self.As Player BP`)) "Hidden")
        (set `PlayerController.bShowMouseCursor` false (`GameplayStatics.GetPlayerController` 0))
        (switch `string` _returnvalue_2
          (:`LB`
            (bind _returnvalue_3 (`|CreateWidget` "/Game/UI/UI_Assets/UIBlueprints/WB_BossIntro_Foredrone.WB_BossIntro_Foredrone_C" _returnvalue))
            (`UserWidget.AddToViewport` _returnvalue_3 0))
          (:`Level_2B`
            (bind _returnvalue_4 (`|CreateWidget` "/Game/UI/UI_Assets/UIBlueprints/WB_BossIntro_Pylonator.WB_BossIntro_Pylonator_C" _returnvalue))
            (`UserWidget.AddToViewport` _returnvalue_4 0))
          (:`Level_3B`
            (bind _returnvalue_5 (`|CreateWidget` "/Game/UI/UI_Assets/UIBlueprints/WB_BossIntro_GrubberGuy.WB_BossIntro_GrubberGuy_C" _returnvalue))
            (`UserWidget.AddToViewport` _returnvalue_5 0)))
        (`KismetSystemLibrary.Delay` 2.8)
        (`Widget.RemoveFromParent` _returnvalue_3)
        (`Widget.RemoveFromParent` _returnvalue_4)
        (`Widget.RemoveFromParent` _returnvalue_5)
        (set `/Game/Characters/Player/PlayerBP.IsPlayerCotrollerEnabled?` true _as_player_bp)
        (`Widget.SetVisibility` (`/Game/Characters/Player/PlayerBP.HeadsUpDisplayRef` (`self.As Player BP`)) "Visible")
        (set `PlayerController.bShowMouseCursor` true (`GameplayStatics.GetPlayerController` 0))))))

(fn `UserConstructionScript`)