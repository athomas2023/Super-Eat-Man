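; AI controller for the Globber NPC that runs its behavior tree and fires projectiles at the player.
; Sight perception updates set or clear the TargetActor blackboard key.
; After a short delay, any player sight update, including sight loss, turns the pawn toward the player and spawns a targeted BP_ProjectileBase at its FireLocation.
; A separate Fire function spawning DroneProjectile_BP is not called within this graph.
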(event `self.ReceiveBeginPlay`
  ;[1 0.244 0.9526] Globber Brain
  (`self.RunBehaviorTree` "/Game/Characters/NPC/Globber/BT_Globber.BT_Globber"))

(event `self.AIPerception.OnTargetPerceptionUpdated`
  (params (Actor :type "Actor Object Reference") (Stimulus :type "AIStimulus Structure"))
  ;[1 0.244 0.9526] Globber Brain
  ;;[1 1 1] If SEM is in Globber Sight, Pass True to Fire Volly Projectile
  (bind _sem_in_attack_range (`self.Handle Sight Sense` Actor Stimulus))
  (`KismetSystemLibrary.Delay` 0.5)
  (`self.Globber Volly` _sem_in_attack_range Actor))

(fn `Fire`
  (bind _mesh (`Character.Mesh` (`self.Globber New Ref`)))
  ;[1 1 1] Shooting
  (`SceneComponent.K2_SetWorldRotation` _mesh (`KismetMathLibrary.FindLookAtRotation` (`SceneComponent.K2_GetComponentLocation` _mesh) (`SceneComponent.K2_GetComponentLocation` (`Character.Mesh` (`GameplayStatics.GetPlayerCharacter` 0)))) false false)
  (`|SpawnActorFromClass` "/Game/Weapons/DroneProjectile_BP.DroneProjectile_BP_C" (`SceneComponent.K2_GetComponentToWorld` (`Character.Mesh` (`self.Globber New Ref`))) "Undefined" "MultiplyWithRoot" null null null))

(fn `Globber Volly`
  (params (Attack :type Boolean) (`Target Actor` :type "Actor Object Reference"))
  (bind _returnvalue (`self.K2_GetPawn` self))
  ;[1 1 1] Globber Set Rotation To SEM
  (if Attack
    (`SceneComponent.K2_SetWorldRotation` (`Actor.RootComponent` _returnvalue) (`KismetMathLibrary.FindLookAtRotation` (`self.K2_GetActorLocation` _returnvalue) (`SceneComponent.K2_GetComponentLocation` (`Character.Mesh` (`GameplayStatics.GetPlayerCharacter` 0)))) false false)
    ;[1 0.03119 0.899] Test** Option for Spawning Projectile from Globber Fire Location (Arrow Component)
    (bind _asbp_globber_new (cast `/Game/Characters/NPC/Globber/BP_GlobberNew` (`self.K2_GetPawn` self)))
    (bind _fire_location (`/Game/Characters/NPC/Globber/BP_GlobberNew.Fire Location` _asbp_globber_new))
    ;[1 1 1] Spawn Projectile at Globber Location
    (`|SpawnActorFromClass` "/Game/Weapons/BP_ProjectileBase.BP_ProjectileBase_C" (`KismetMathLibrary.MakeTransform` (`SceneComponent.K2_GetComponentLocation` _fire_location) (`SceneComponent.K2_GetComponentRotation` _fire_location)) "Undefined" "MultiplyWithRoot" null `Target Actor` 1.5 3000.0 null)))

(fn `Handle Sight Sense`
  (params (Actor :type "Actor Object Reference") (Stimulus :type "AIStimulus Structure"))
  (returns (`SEM in Attack Range` :type Boolean))
  (bind (_stimulus_age _stimulus_expirationage _stimulus_strength _stimulus_stimuluslocation _stimulus_receiverlocation _stimulus_tag _stimulus_bsuccessfullysensed) (break `AIStimulus` (`local.Stimulus`)))
  (bind _returnvalue (`AIPerceptionSystem.GetSenseClassForStimulus` Stimulus))
  (if (== _returnvalue "/Script/AIModule.AISense_Sight")
    (if (== (`local.Actor`) (`GameplayStatics.GetPlayerCharacter` 0))
      (`BlackboardComponent.SetValueAsObject` (`self.Blackboard`) "TargetActor" (`KismetMathLibrary.SelectObject` (`GameplayStatics.GetPlayerCharacter` 0) null _stimulus_bsuccessfullysensed))
      (return true)
      (else
        (return false)))
    (else
      (return false))))

(fn `UserConstructionScript`)