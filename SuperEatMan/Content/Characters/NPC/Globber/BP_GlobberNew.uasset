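; BP_GlobberNew is the Globber NPC, a robot enemy that takes damage, shows lock-on highlighting and is destroyed at zero health.
; TakeDamage flashes a damage overlay, plays sound and Niagara effects, decrements Health and explodes the actor on death.
; DamagedByBully and DamagedByWiseGuy apply heavier and single-point damage respectively, while DisplayLock and DisableLock toggle the lock-on overlay.
; Spline movement and look-at events are empty stubs, with disconnected draft logic for them and projectile firing.
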(event `/Game/Characters/NPC/Enemies/I_Enemy.TakeDamage`
  (params (BaseDamage :type "Float (double-precision)"))
  ;[1 1 1] Will be Replaced with Spark VFX
  (`MeshComponent.SetOverlayMaterial` (`self.Body`) "/Game/Characters/NPC/M_DamageOverlay.M_DamageOverlay")
  (`KismetSystemLibrary.Delay` 0.3)
  (`MeshComponent.SetOverlayMaterial` (`self.Body`) null)
  (`GameplayStatics.PlaySoundAtLocation` "/Game/Sound/SFX/RobotDamaged.RobotDamaged" (`SceneComponent.K2_GetComponentLocation` (`self.Body`)) (struct) 1.0 1.0 0.0 null null null null)
  (`NiagaraFunctionLibrary.SpawnSystemAtLocation` "/Game/Weapons/FX_WiseGuy.FX_WiseGuy" (`SceneComponent.K2_GetComponentLocation` (`self.Body`)) (struct :`Roll` 90.0) (0.01 0.01 0.01))
  (bind _result (`/Engine/EditorBlueprintResources/StandardMacros.DecrementInt` (`self.Health`))
    (:`  `
      (if (<= _result 0)
        (`NiagaraFunctionLibrary.SpawnSystemAtLocation` "/Game/Effects/VFX/NS/Explod.Explod" (`SceneComponent.K2_GetComponentLocation` (`self.Body`)) (struct :`Roll` 90.0))
        (`self.K2_DestroyActor`)))))

(event `/Game/Characters/NPC/Enemies/I_Enemy.DisplayLock`
  (`MeshComponent.SetOverlayMaterial` (`self.Body`) "/Game/Characters/NPC/M_LockOnOverlay.M_LockOnOverlay"))

(event `/Game/Characters/NPC/Enemies/I_Enemy.DisableLock`
  (`MeshComponent.SetOverlayMaterial` (`self.Body`) null))

(event `Move Along Spline`
  ;[1 1 1] Movement Alone Spline
)

(event `Look at Target`
  ;[1 1 1] Look at Target
)

(fn `Damaged By Bully`
  (returns (`Enemy Destroyed` :type Boolean))
  (bind _output_get (set `self.Health` (- (`self.Health`) 3)))
  (bind _returnvalue (<= _output_get 0))
  (if _returnvalue
    (`self.K2_DestroyActor`)
    (`NiagaraFunctionLibrary.SpawnSystemAtLocation` "/Game/Weapons/FX_WiseGuy.FX_WiseGuy" (`self.K2_GetActorLocation`))
    (return _returnvalue)))

(fn `Damaged by Wise Guy`
  (returns (`Enemy Destroyed?` :type Boolean) (`Obstacle Destroyed?` :type Boolean))
  (bind _returnvalue (`self.K2_GetActorLocation`))
  (bind _result (`/Engine/EditorBlueprintResources/StandardMacros.DecrementInt` (`self.Health`))
    (:`  `
      (bind _returnvalue_2 (<= _result 0))
      (if _returnvalue_2
        (`self.K2_DestroyActor`)
        (`GameplayStatics.PlaySoundAtLocation` "/Game/Sound/SFX/RobotDamaged.RobotDamaged" _returnvalue (struct) 1.0 1.0 0.0 null null null null)
        (`NiagaraFunctionLibrary.SpawnSystemAtLocation` "/Game/Weapons/FX_WiseGuy.FX_WiseGuy" _returnvalue)
        (return _returnvalue_2 false)))))

(fn `UserConstructionScript`)