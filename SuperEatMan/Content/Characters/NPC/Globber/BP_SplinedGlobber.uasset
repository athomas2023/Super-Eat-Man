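; Globber NPC that travels along a spline and attacks the player on entering its detection area.
; A Timeline, play rate scaled by completion time, moves the rotation pivot along the spline from BeginPlay.
; Overlap starts a self-re-triggering gun look-at loop, then enables attacking after a short delay.
; While attacking, Tick spawns a projectile every frame at the target's location; exit stops firing, but tracking continues.
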(event `self.ReceiveBeginPlay`
  (`self.Move Along Spline`))

(event `self.Detection Area.OnComponentBeginOverlap`
  (params (OverlappedComponent :type "PrimitiveComponent Object Reference") (OtherActor :type "Actor Object Reference") (OtherComp :type "PrimitiveComponent Object Reference") (OtherBodyIndex :type Integer) (bFromSweep :type Boolean) (SweepResult :type "HitResult Structure (by ref)"))
  ;[1 1 1] Position for Attack
  (bind _asplayer_bp (cast `/Game/Characters/Player/PlayerBP` OtherActor))
  (set `self.Targeted Actor` _asplayer_bp)
  (`self.Look at Target`)
  (`KismetSystemLibrary.Delay` 0.5)
  (set `self.Should Attack?` true))

(event `self.Detection Area.OnComponentEndOverlap`
  (params (OverlappedComponent :type "PrimitiveComponent Object Reference") (OtherActor :type "Actor Object Reference") (OtherComp :type "PrimitiveComponent Object Reference") (OtherBodyIndex :type Integer))
  ;[1 1 1] Resume Roam
  (if (== OtherActor (`self.Targeted Actor`))
    (set `self.Should Attack?` false)))

(event `self.ReceiveTick`
  (params (DeltaSeconds :type "Float (single-precision)"))
  (bind _targeted_actor (`self.Targeted Actor`))
  ;[1 1 1] Toggling Attack
  (if (`self.Should Attack?`)
    (`|SpawnActorFromClass` "/Game/Weapons/BP_ProjectileBase.BP_ProjectileBase_C" (`KismetMathLibrary.MakeTransform` (`self.K2_GetActorLocation` _targeted_actor)) "Undefined" "MultiplyWithRoot" null _targeted_actor 1.0 2000.0 null)))

(event `Move Along Spline`
  ;[1 1 1] Movement Alone Spline
  (`TimelineComponent.SetPlayRate` (`self.Globber Timeline`) (/ 1.0 (`self.Time To Complate`)))
  (bind (_direction _movement_track) (`Timeline|Globber Timeline`) ; Ensure Length is Set to 1 - else play rate will not work as intended
    (:`Update`
      (bind _returnvalue_location (`KismetMathLibrary.BreakTransform` (`SplineComponent.GetTransformAtDistanceAlongSpline` (`self.Spline`) (`KismetMathLibrary.Lerp` 0.0 (`SplineComponent.GetSplineLength` (`self.Spline`)) _movement_track) "Local" false)))
      (`SceneComponent.K2_SetRelativeTransform` (`self.Rotation Piviot`) (`KismetMathLibrary.MakeTransform` _returnvalue_location (struct) (2.0 2.0 2.0)) false false))))

(event `Look at Target`
  (bind _gun (`self.Gun`))
  ;[1 1 1] Look at Target
  (`/Engine/EditorBlueprintResources/StandardMacros.IsValid` (`self.Targeted Actor`)
    (:`Is Valid`
      (`SceneComponent.K2_SetRelativeRotation` (`self.Gun`) (`KismetMathLibrary.RInterpTo` (`SceneComponent.K2_GetComponentRotation` _gun) (`KismetMathLibrary.FindLookAtRotation` (`SceneComponent.K2_GetComponentLocation` _gun) (`self.K2_GetActorLocation` (`self.Targeted Actor`))) (`GameplayStatics.GetWorldDeltaSeconds`)) false false)
      (`KismetSystemLibrary.Delay` 0.001)
      (`self.Look at Target`))))

(fn `UserConstructionScript`)