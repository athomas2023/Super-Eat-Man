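; ZapJack NPC, apparently a robot enemy, that takes damage from Bully and Wise Guy attacks and is destroyed when its health runs out.
; Bully hits remove more health than Wise Guy hits; both deaths spawn the Wise Guy effect and report destruction, but only Wise Guy kills play a sound.
; Tick runs a persistently drawn debug object trace from FireLocation, with an end point that scales world position rather than direction, and does nothing on a hit.
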(event `self.ReceiveTick`
  (params (DeltaSeconds :type "Float (single-precision)"))
  (bind _fire_location (`self.Fire Location`))
  (bind _returnvalue (`SceneComponent.K2_GetComponentLocation` _fire_location))
  (bind _outhit (`KismetSystemLibrary.LineTraceSingleForObjects` :`Start` (+ (`SceneComponent.GetForwardVector` _fire_location) _returnvalue) :`End` (* _returnvalue (`self.Projectile Distance`)) :`ObjectTypes` (`self.Object Types`) :`DrawDebugType` "Persistent"))
  (if (`GameplayStatics.BreakHitResult` _outhit)
    _))

(fn `Damaged By Bully`
  (returns (`Enemy Destroyed` :type Boolean))
  (bind _output_get (set `self.Health` (- (`self.Health`) 3)))
  (bind _returnvalue (<= _output_get 0))
  (if _returnvalue
    (`self.K2_DestroyActor`)
    (`NiagaraFunctionLibrary.SpawnSystemAtLocation` "/Game/Weapons/FX_WiseGuy.FX_WiseGuy" (`self.K2_GetActorLocation`))
    (return _returnvalue)))

(fn `Damaged by Wise Guy`
  (returns (`Enemy Destroyed?` :type Boolean) (`Obstacle Destroyed?` :type Boolean))
  (bind _returnvalue (`self.K2_GetActorLocation`))
  (bind _result (`/Engine/EditorBlueprintResources/StandardMacros.DecrementInt` (`self.Health`))
    (:`  `
      (bind _returnvalue_2 (<= _result 0))
      (if _returnvalue_2
        (`self.K2_DestroyActor`)
        (`GameplayStatics.PlaySoundAtLocation` "/Game/Sound/SFX/RobotDamaged.RobotDamaged" _returnvalue (struct) 1.0 1.0 0.0 null null null null)
        (`NiagaraFunctionLibrary.SpawnSystemAtLocation` "/Game/Weapons/FX_WiseGuy.FX_WiseGuy" _returnvalue)
        (return _returnvalue_2 false)))))

(fn `UserConstructionScript`)