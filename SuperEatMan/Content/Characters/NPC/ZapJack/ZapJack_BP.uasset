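; ZapJack is an NPC enemy that fires a projectile at the player when the player overlaps its detection area.
; The overlap spawns a zero-gravity BP_ZapjackProjectile at the arrow's location with the player as target, after a line trace whose result is unused.
; Separate damage functions for Bully and Wise Guy hits reduce health, destroying the actor with a Niagara effect at zero, plus a sound for Wise Guy.
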(event `self.Detection Area.OnComponentBeginOverlap`
  (params (OverlappedComponent :type "PrimitiveComponent Object Reference") (OtherActor :type "Actor Object Reference") (OtherComp :type "PrimitiveComponent Object Reference") (OtherBodyIndex :type Integer) (bFromSweep :type Boolean) (SweepResult :type "HitResult Structure (by ref)"))
  (bind _returnvalue (`SceneComponent.K2_GetComponentLocation` (`self.Arrow`)))
  (bind _asplayer_bp (cast `/Game/Characters/Player/PlayerBP` OtherActor))
  (`KismetSystemLibrary.LineTraceSingleForObjects` _returnvalue (* (`SceneComponent.GetRightVector` (`self.Arrow`)) (`self.Projectile Distance`)) (`self.Object Types`))
  (`|SpawnActorFromClass` "/Game/Weapons/BP_ZapjackProjectile.BP_ZapjackProjectile_C" (`KismetMathLibrary.MakeTransform` _returnvalue) "Undefined" "MultiplyWithRoot" null _asplayer_bp 0.0 2000.0 null))

(fn `Damaged By Bully`
  (returns (`Enemy Destroyed` :type Boolean))
  (bind _output_get (set `self.Health` (- (`self.Health`) 3)))
  (if (<= _output_get 0)
    (`self.K2_DestroyActor`)
    (`NiagaraFunctionLibrary.SpawnSystemAtLocation` "/Game/Weapons/FX_WiseGuy.FX_WiseGuy" (`self.K2_GetActorLocation`))
    (return false)))

(fn `Damaged by Wise Guy`
  (returns (`Enemy Destroyed?` :type Boolean) (`Obstacle Destroyed?` :type Boolean))
  (bind _returnvalue (`self.K2_GetActorLocation`))
  (bind _result (`/Engine/EditorBlueprintResources/StandardMacros.DecrementInt` (`self.Health`))
    (:`  `
      (bind _returnvalue_2 (<= _result 0))
      (if _returnvalue_2
        (`self.K2_DestroyActor`)
        (`GameplayStatics.PlaySoundAtLocation` "/Game/Sound/SFX/RobotDamaged.RobotDamaged" _returnvalue (struct) 1.0 1.0 0.0 null null null null)
        (`NiagaraFunctionLibrary.SpawnSystemAtLocation` "/Game/Weapons/FX_WiseGuy.FX_WiseGuy" _returnvalue)
        (return _returnvalue_2 false)))))

(fn `UserConstructionScript`)