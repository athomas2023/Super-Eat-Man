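; BP_Globber is a flying drone enemy that shoots projectiles at the player character and awards a GrindPoint when its health runs out.
; Movement lerps the body toward randomly picked location points via a timer, re-picking after short random delays.
; Shooting aims an arrow at the player's mesh and spawns DroneProjectile_BP.
; Both loops start in the respawn handler, but its binding is disconnected, as is the older startup chain; BeginPlay only caches the player.
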(event `self.ReceiveBeginPlay`
  (bind _asplayer_bp (cast `/Game/Characters/Player/PlayerBP` (`GameplayStatics.GetPlayerCharacter` 0)))
  (set `self.New Player BP Ref` _asplayer_bp))

(event `self.ReceiveTick`
  (params (DeltaSeconds :type "Float (single-precision)"))
  ;[1 1 1] Enemy Death
)

(event `Shoot`
  (bind _arrow (`self.Arrow`))
  ;[1 1 1] Shooting
  (`SceneComponent.K2_SetWorldRotation` _arrow (`KismetMathLibrary.FindLookAtRotation` (`SceneComponent.K2_GetComponentLocation` _arrow) (`SceneComponent.K2_GetComponentLocation` (`Character.Mesh` (`self.Current Character`)))) false false)
  (`|SpawnActorFromClass` "/Game/Weapons/DroneProjectile_BP.DroneProjectile_BP_C" (`SceneComponent.K2_GetComponentToWorld` (`self.Arrow`)) "Undefined" "MultiplyWithRoot" null null null))

(event `OnPossessedPawnChanged_Event`
  (params (OldPawn :type "Pawn Object Reference") (NewPawn :type "Pawn Object Reference"))
  ;[1 1 1] Get Player Character
  (bind _asplayer_bp (cast `/Game/Characters/Player/PlayerBP` NewPawn))
  (bind _output_get (set `self.Current Character` _asplayer_bp))
  (add `self.OnDestroyed` _output_get (delegate `Spawn`)))

(event `Spawn` :!signature `self.OnDestroyed`
  (params (DestroyedActor :type "Actor Object Reference"))
  ;[1 1 1] Handle Respawn
  (`Controller.Possess` (`GameplayStatics.GetPlayerController` 0) null)
  (`self.FindNextLocation`)
  (`self.Shoot` :!label _label)
  (`KismetSystemLibrary.Delay` 2.0)
  (goto _label))

(event `Moving`
  (bind _body (`self.Body`))
  ;[1 1 1] Update Moving
  (set `self.Alpha` 0.0)
  (`KismetSystemLibrary.K2_SetTimerDelegate` (delegate `Moving`) 0.02)
  (set `self.Alpha` (+ (`self.Alpha`) 0.02))
  (`SceneComponent.K2_SetWorldLocation` _body (`KismetMathLibrary.VLerp` (`SceneComponent.K2_GetComponentLocation` _body) (`self.LocationToMove`) (`self.Alpha`)) false false))

(event `FindNextLocation`
  (bind _array (`|MakeArray` null null null null null null :!type "ArrowComponent Object Reference"))
  ;[1 1 1] Cycle Movement Patterns
  (set `self.LocationToMove` (`SceneComponent.K2_GetComponentLocation` (`|GetArrayItem` _array (`KismetMathLibrary.RandomIntegerInRange` 0 (`KismetArrayLibrary.Array_LastIndex` _array)))))
  (`self.Moving`)
  (`KismetSystemLibrary.Delay` (`KismetMathLibrary.RandomFloatInRange` 0.5 1.0))
  (`self.FindNextLocation`))

(event `Damage Taken`
  ;[1 1 1] Death
  (bind _result (`/Engine/EditorBlueprintResources/StandardMacros.DecrementInt` (`self.EnemyHealth`))
    (:`  `
      (if (<= _result 0)
        (`/Game/Characters/Player/PlayerBP.GrindPoint` (`self.New Player BP Ref`))
        (`self.K2_DestroyActor`)))))

(fn `UserConstructionScript`)