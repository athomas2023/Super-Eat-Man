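; Spline path actor for the Foredrone boss, moving a referenced actor along the path from the first point to the last.
; BeginPlay registers the spline with the boss and caches the player.
; StartBoss scales timeline rate by spline length and player max speed to match pace, with updates setting location and tangent-based rotation, yaw flipped 180°.
; Construction snaps the actor to the first point; helpers stop the timeline or store its position.
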(event `self.ReceiveBeginPlay`
  ;[1 1 1] Boss Ref
  (bind _asbp_foredrone (cast `/Game/Characters/NPC/Foredrone/BP_Foredrone` (`self.Actor`)))
  (set `/Game/Characters/NPC/Foredrone/BP_Foredrone.As BP Foredrone Spline` self _asbp_foredrone)
  (bind _asplayer_bp (cast `/Game/Characters/Player/PlayerBP` (`GameplayStatics.GetPlayerCharacter` 0)))
  (set `self.As Player BP` _asplayer_bp))

(event `StartBoss`
  ;[1 1 1] Start Boss
  (`TimelineComponent.SetPlayRate` (`self.Timeline`) (/ 1.0 (/ (`SplineComponent.GetSplineLength` (`self.Spline`)) (`MovementComponent.GetMaxSpeed` (`Character.CharacterMovement` (`self.As Player BP`))))))
  (`self.Play Timeline`))

(event `Play Timeline`
  ;[1 1 1] Start & Stop Timeline
  (`TimelineComponent.Play` (`self.Timeline`)))

(event `StopTimeline`
  ;[1 1 1] Start & Stop Timeline
  (`TimelineComponent.Stop` (`self.Timeline`)))

(fn `Store Playback Position`
  (set `self.PlaybackPosition` (`TimelineComponent.GetPlaybackPosition` (`self.Timeline`))))

(fn `UserConstructionScript`
  (`self.K2_SetActorLocation` (`self.Actor`) (`SplineComponent.GetLocationAtSplinePoint` (`self.Spline`) 0 "World") false false))