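; Foredrone NPC that travels along a spline and aims a Niagara laser at the player inside its detection area.
; A timeline scaled by TimeToComplete drives the spline movement.
; Overlap starts a self-repeating delayed look-at and, after a short delay, enables attack; leaving disables only the attack.
; While attacking, Tick runs a debug-drawn line trace to place the beam and impact effects, without applying damage.
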(event `self.ReceiveBeginPlay`
  ;[0.0319 1 0] Begin Play
  ;;[1 1 1] Disable Laser Visibility
  (`SceneComponent.SetVisibility` (`self.Niagara Laser`) false false)
  (`SceneComponent.SetVisibility` (`self.Niagara Laser Impact`) false false)
  (`FXSystemComponent.SetColorParameter` (`self.Niagara Laser`) "Color" (struct :`R` 1.0 :`B` 0.029524 :`A` 1.0))
  (`FXSystemComponent.SetColorParameter` (`self.Niagara Laser Impact`) "Color" (struct :`R` 1.0 :`B` 0.029524 :`A` 1.0))
  (`self.Move Along Spline`))

(event `self.Detection Area.OnComponentBeginOverlap`
  (params (OverlappedComponent :type "PrimitiveComponent Object Reference") (OtherActor :type "Actor Object Reference") (OtherComp :type "PrimitiveComponent Object Reference") (OtherBodyIndex :type Integer) (bFromSweep :type Boolean) (SweepResult :type "HitResult Structure (by ref)"))
  ;[1 1 1] Position for Attack
  (bind _asplayer_bp (cast `/Game/Characters/Player/PlayerBP` OtherActor))
  (set `self.Targeted Actor` _asplayer_bp)
  (`self.Look at Target`)
  (`KismetSystemLibrary.Delay` 0.5)
  (set `self.Should Attack?` true))

(event `self.Detection Area.OnComponentEndOverlap`
  (params (OverlappedComponent :type "PrimitiveComponent Object Reference") (OtherActor :type "Actor Object Reference") (OtherComp :type "PrimitiveComponent Object Reference") (OtherBodyIndex :type Integer))
  ;[1 1 1] Resume Roam
  (if (== OtherActor (`self.Targeted Actor`))
    (set `self.Should Attack?` false)))

(event `self.ReceiveTick`
  (params (DeltaSeconds :type "Float (single-precision)"))
  ;[1 1 1] Toggling Attack
  (if (`self.Should Attack?`)
    (`self.Activate Laser Burst`)
    (else
      (`self.Deactivate Laser Burst`))))

(event `Move Along Spline`
  ;[1 1 1] Movement Alone Spline
  (`TimelineComponent.SetPlayRate` (`self.Saucer Timeline`) (/ 1.0 (`self.Time to Complete`)))
  (bind (_direction _movement_track) (`Timeline|Timeline`) ; Ensure Length is Set to 1 - else play rate will not work as intended
    (:`Update`
      (bind _returnvalue_location (`KismetMathLibrary.BreakTransform` (`SplineComponent.GetTransformAtDistanceAlongSpline` (`self.Spline`) (`KismetMathLibrary.Lerp` 0.0 (`SplineComponent.GetSplineLength` (`self.Spline`)) _movement_track) "Local" false)))
      (`SceneComponent.K2_SetRelativeTransform` (`self.Rotation Piviot`) (`KismetMathLibrary.MakeTransform` _returnvalue_location (struct) (2.0 2.0 2.0)) false false))))

(event `Look at Target`
  (bind _skeletalmesh (`self.SkeletalMesh`))
  ;[1 1 1] Look at Target
  (`/Engine/EditorBlueprintResources/StandardMacros.IsValid` (`self.Targeted Actor`)
    (:`Is Valid`
      (`SceneComponent.K2_SetRelativeRotation` (`self.SkeletalMesh`) (`KismetMathLibrary.RInterpTo` (`SceneComponent.K2_GetComponentRotation` _skeletalmesh) (`KismetMathLibrary.FindLookAtRotation` (`SceneComponent.K2_GetComponentLocation` _skeletalmesh) (`self.K2_GetActorLocation` (`self.Targeted Actor`))) (`GameplayStatics.GetWorldDeltaSeconds`)) false false)
      (`KismetSystemLibrary.Delay` 0.001)
      (`self.Look at Target`))))

(event `Activate Laser Burst`
  (bind _skeletalmesh (`self.SkeletalMesh`))
  ;[1 1 1] Fire Laser
  (bind _outhit (`KismetSystemLibrary.LineTraceSingle` :`Start` (+ (`SceneComponent.K2_GetComponentLocation` _skeletalmesh) (`SceneComponent.GetForwardVector` _skeletalmesh)) :`End` (* (- (`self.K2_GetActorLocation` (`self.Targeted Actor`)) (`SceneComponent.K2_GetComponentLocation` (`self.SkeletalMesh`))) (`self.Attack Distance`)) :`TraceChannel` "TraceTypeQuery3" :`DrawDebugType` "ForOneFrame"))
  (set `self.Blocked Hit` (`GameplayStatics.BreakHitResult` _outhit))
  (set `self.Hit Location` (`.Location` (`GameplayStatics.BreakHitResult` _outhit)))
  (`SceneComponent.SetVisibility` (`self.Niagara Laser`) (`self.Blocked Hit`) false)
  (`FXSystemComponent.SetVectorParameter` (`self.Niagara Laser`) "LaserEnd" (`self.Hit Location`))
  (`SceneComponent.SetVisibility` (`self.Niagara Laser Impact`) (`self.Blocked Hit`) false)
  (`SceneComponent.K2_SetWorldLocation` (`self.Niagara Laser Impact`) (`self.Hit Location`) false false))

(event `Deactivate Laser Burst`
  ;[1 1 1] Cancel Laser
  (`SceneComponent.SetVisibility` (`self.Niagara Laser`) false false)
  (`SceneComponent.SetVisibility` (`self.Niagara Laser Impact`) false false))

(fn `UserConstructionScript`)