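; BP_TutorialText is a child Blueprint that reacts once when the player character overlaps it, apparently to show timed tutorial text.
; On that first overlap it runs the parent's overlap logic, then sets the narration UI's hold time from its TextDuration variable.
; BeginPlay and construction only call the parent, and Tick is disabled.
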(event `self.ReceiveBeginPlay`
  (`parent.ReceiveBeginPlay`))

(event `self.ReceiveActorBeginOverlap`
  (params (OtherActor :type "Actor Object Reference"))
  (if (== OtherActor (`GameplayStatics.GetPlayerCharacter` 0))
    (`/Engine/EditorBlueprintResources/StandardMacros.DoOnce` false
      (:`Completed`
        (`parent.ReceiveActorBeginOverlap` OtherActor)
        (set `/Game/Sound/Soundfont/WB_SoundfontDemo.HoldTime` (`self.TextDuration`) (`self.NarrationUI`))))))

(fn `UserConstructionScript`
  (`parent.UserConstructionScript`))