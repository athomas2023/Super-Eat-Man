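; BP_Dissolve_Static is an actor that plays a dissolve effect on a static mesh with matching Niagara particles.
; A setup macro, run at construction and in UpdateData, pushes alpha, boosted edge color and dissolve texture to both, creating dynamic material instances per slot.
; BeginPlay calls UpdateData, whose timeline then animates the shared Alpha parameter on materials and particle system together.
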(event `self.ReceiveBeginPlay`
  (`self.Update Data`))

(event `Update Data`
  (`self.StaticMesh_Setup_Macro` (`self.Niagara`) (`self.StaticMesh`)
    (:`Completed`
      (bind (_direction _newtrack_0) (`Timeline|Timeline`)
        (:`Update`
          (`MeshComponent.SetScalarParameterValueOnMaterials` (`self.StaticMesh`) "Alpha" _newtrack_0)
          (`NiagaraComponent.SetVariableFloat` (`self.Niagara`) "Alpha" _newtrack_0))))))

(fn `UserConstructionScript`
  (`self.StaticMesh_Setup_Macro` (`self.Niagara`) (`self.StaticMesh`)))