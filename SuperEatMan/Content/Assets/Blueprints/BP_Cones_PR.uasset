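; BP_Cones_PR is a destructible cone obstacle that removes itself from the level.
; DestroyCOne and DestroyBarrel simply destroy the actor.
; DamagedByWiseGuy also spawns a half-scale particle effect at its location and reports an obstacle, not an enemy, as destroyed.
; DamageTaken is empty, and the health decrement and player GrindPoint call are disconnected.
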(event `Destroy COne`
  ;[1 1 1] Death
  (`self.K2_DestroyActor`))

(event `Damage Taken`)

(fn `Damaged by Wise Guy`
  (returns (`Enemy Destroyed?` :type Boolean) (`Obstacle Destroyed?` :type Boolean))
  (`self.K2_DestroyActor`)
  (`GameplayStatics.SpawnEmitterAtLocation` "/Engine/Tutorial/SubEditors/TutorialAssets/TutorialParticleSystem.TutorialParticleSystem" (`self.K2_GetActorLocation`) (struct) (0.5 0.5 0.5))
  (return false true))

(fn `Destroy Barrel`
  (`self.K2_DestroyActor`))

(fn `UserConstructionScript`)