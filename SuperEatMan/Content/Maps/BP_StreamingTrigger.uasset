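; Trigger volume Blueprint that streams levels in and out when something begins overlapping its Box, with no filter on the overlapping actor.
; It asynchronously loads the level named in LevelToMakeVisible, visible after load, and unloads the one named in LevelToHide.
; Each step is skipped if its name is None or the level is already in the desired state.
; An unconnected alternative that only toggles level visibility never runs.
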(event `self.Box.OnComponentBeginOverlap`
  (params (OverlappedComponent :type "PrimitiveComponent Object Reference") (OtherActor :type "Actor Object Reference") (OtherComp :type "PrimitiveComponent Object Reference") (OtherBodyIndex :type Integer) (bFromSweep :type Boolean) (SweepResult :type "HitResult Structure (by ref)"))
  (bind _level_to_make_visible (`self.Level To Make Visible`))
  (bind _level_to_hide (`self.Level To Hide`))
  (`|ExecutionSequence`
    (:`then_0`
      (if (== _level_to_make_visible "None")
        _
        (elif (not (`LevelStreaming.IsLevelLoaded` (`GameplayStatics.GetStreamingLevel` _level_to_make_visible)))
          (`GameplayStatics.LoadStreamLevel` _level_to_make_visible true))))
    (:`then_1`
      (if (== _level_to_hide "None")
        _
        (elif (`LevelStreaming.IsLevelLoaded` (`GameplayStatics.GetStreamingLevel` _level_to_hide))
          (`GameplayStatics.UnloadStreamLevel` _level_to_hide))))))

(fn `UserConstructionScript`)