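; One-shot narration trigger actor that shows on-screen story text when the player overlaps it.
; It creates a WB_NarrativeText widget with either its own DisplayText or the next line consumed from BP_Narration_Controller's Narration queue, falling back to DisplayText if none is available.
; FormatNarration replaces "\n" sequences in the text, and after a fixed delay the widget is removed and the trigger destroys itself.
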(event `self.ReceiveActorBeginOverlap`
  (params (OtherActor :type "Actor Object Reference"))
  (cast `/Game/Characters/Player/PlayerBP` OtherActor)
  (bind _returnvalue (`|CreateWidget` "/Game/UI/UI_Assets/UIBlueprints/WB_NarrativeText.WB_NarrativeText_C"))
  (bind _output_get (set `self.Narration` _returnvalue))
  (if (`self.TextSet`)
    (set `/Game/UI/UI_Assets/UIBlueprints/WB_NarrativeText.Text` (`self.FormatNarration` (`self.DisplayText`)) _output_get :!label _label)
    (else
      (bind _returnvalue_2 (`GameplayStatics.GetActorOfClass` "/Game/Gameplay/StoryElements/BP_Narration_Controller.BP_Narration_Controller_C"))
      (bind _asbp_narration_controller (cast `/Game/Gameplay/StoryElements/BP_Narration_Controller` _returnvalue_2)
        (:`then`
          (bind _narration (`/Game/Gameplay/StoryElements/BP_Narration_Controller.Narration` _asbp_narration_controller))
          (if (`KismetArrayLibrary.Array_IsValidIndex` _narration)
            (set `/Game/UI/UI_Assets/UIBlueprints/WB_NarrativeText.Text` (`self.FormatNarration` (`|GetArrayItem` _narration)) _output_get)
            (`KismetArrayLibrary.Array_Remove` _narration)
            (else
              (goto _label))))
        (:`CastFailed`
          (goto _label)))))
  (`UserWidget.AddToViewport` _output_get 0)
  (`KismetSystemLibrary.Delay` 10.0)
  (`Widget.RemoveFromParent` (`self.Narration`))
  (`self.K2_DestroyActor`))

(fn `FormatNarration`
  (params (Text :type String))
  (returns (NewParam :type String))
  (return (`KismetStringLibrary.Replace` Text "\\n" " \n")))

(fn `UserConstructionScript`)