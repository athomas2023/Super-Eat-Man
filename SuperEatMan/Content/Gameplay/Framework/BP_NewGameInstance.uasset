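; Game instance that holds and persists game settings, level unlocks, coins and character unlocks through BP_SaveGameObject in slot "SEM Save 1".
; SEM save/load functions copy instance variables to and from disk; each save writes a fresh object, overwriting fields it omits.
; Deprecated Init loads or creates the save and applies the base sound mix.
; Older PlayerData functions bank PlayerBP coins, save workshop purchases or clear the slot.
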(event `Init SEM`
  ;[1 0 0.1231] Depreciated
)

(event `Save HUD Data`
  ;[1 0 0.1231] Depreciated
)

(event `self.ReceiveInit`
  (bind _in_sound_mix (`self.In Sound Mix`))
  ;[1 0 0.1231] Depreciated - Managed through "SEM Functions"
  ;;[1 1 1] Check for Selected File (Save Slot Name) in Save Game Object Folder
  (bind _returnvalue (`GameplayStatics.DoesSaveGameExist` "SEM Save 1"))
  (if _returnvalue
    ;;[1 1 1] False: Create Object & Set Ref
    ;; True: Load & Cast, the Set Ref
    (bind _returnvalue_2 (`GameplayStatics.LoadGameFromSlot` "SEM Save 1"))
    (bind _asbp_save_game_object (cast `/Game/Gameplay/Framework/BP_SaveGameObject` _returnvalue_2))
    (bind _output_get (set `self.Save Game Data` _asbp_save_game_object))
    (bind _output_get_2 (set `/Game/Gameplay/Framework/BP_SaveGameObject.Player Data` (struct) _output_get))
    (set `self.Player Data` _output_get_2)
    (else
      (bind _returnvalue_3 (`GameplayStatics.CreateSaveGameObject` "/Game/Gameplay/Framework/BP_SaveGameObject.BP_SaveGameObject_C"))
      (bind _output_get_3 (set `self.Save Game Data` _returnvalue_3))
      (bind _output_get_4 (set `/Game/Gameplay/Framework/BP_SaveGameObject.Player Data` (struct) _output_get_3))
      (set `self.Player Data` _output_get_4)))
  (`KismetSystemLibrary.Delay` 0.1)
  (`GameplayStatics.SetBaseSoundMix` _in_sound_mix)
  ;[1 1 1] This Gets the Information about the sound mix being used in what might be the most convoluded way possible. Will be simplified once audio save is implemented
  (set `self.TestMasterVolume` (`.VolumeAdjuster` (break `SoundClassAdjuster` (`|GetArrayItem` (`SoundMix.SoundClassEffects` _in_sound_mix)))))
  (set `self.TestMusicVolume` (`.VolumeAdjuster` (break `SoundClassAdjuster` (`|GetArrayItem` (`SoundMix.SoundClassEffects` _in_sound_mix) 1))))
  (set `self.TestSFXVolume` (`.VolumeAdjuster` (break `SoundClassAdjuster` (`|GetArrayItem` (`SoundMix.SoundClassEffects` _in_sound_mix) 2)))))

(fn `Clear SEM Data`
  (`GameplayStatics.DeleteGameInSlot` "SEM Save 1"))

(fn `Load Player Data`
  (locals (`Player Ref` :type "/Game/Characters/Player/PlayerBP Object Reference"))
  (bind (_player_data_coinbank _player_data_haswatchedintro_ _player_data_level2unlocked_ _player_data_level3unlocked_ _player_data_mastervolume _player_data_musicvolume _player_data_sfxvolume _player_data_unlockedheckler_ _player_data_unlockedbully_ _player_data_setwiseguy _player_data_setbully _player_data_wiseguyinventorytext _player_data_bullyinventorytext _player_data_highestrank) (break `/Game/Gameplay/Framework/PlayerSaveData` (`/Game/Gameplay/Framework/BP_SaveGameObject.Player Data` (`self.Save Game Data`))))
  (bind _asplayer_bp (cast `/Game/Characters/Player/PlayerBP` (`GameplayStatics.GetPlayerCharacter` 0)))
  (bind _output_get (set `local.Player Ref` _asplayer_bp))
  (set `/Game/Characters/Player/PlayerBP.CoinsCollected` _player_data_coinbank _output_get)
  (set `/Game/Characters/Player/PlayerBP.Rank` _player_data_highestrank _output_get))

(fn `Load SEM Game Settings`
  (returns (`ShouldSkipIntro?` :type Boolean))
  ;[1 0.03119 0.899] Load Game Settings Test
  (bind _returnvalue (`GameplayStatics.DoesSaveGameExist` "SEM Save 1"))
  (if _returnvalue
    (bind _returnvalue_2 (`GameplayStatics.LoadGameFromSlot` "SEM Save 1"))
    (bind _asbp_save_game_object (cast `/Game/Gameplay/Framework/BP_SaveGameObject` _returnvalue_2))
    ;;[1 1 1] Global Player Settings
    (bind _output_get (set `self.SkipOpeningSequence?` (`/Game/Gameplay/Framework/BP_SaveGameObject.SkipOpeningSequence?` _asbp_save_game_object)))
    (set `self.Enable Cell Shader?` (`/Game/Gameplay/Framework/BP_SaveGameObject.Cell Shader Setting` _asbp_save_game_object))
    (set `self.EnableHaptics?` (`/Game/Gameplay/Framework/BP_SaveGameObject.EnableHaptics?` _asbp_save_game_object))
    (set `self.Input Sensitivity Override` (`/Game/Gameplay/Framework/BP_SaveGameObject.Input Sensitivity Override` _asbp_save_game_object))
    (set `self.Enable Gore?` (`/Game/Gameplay/Framework/BP_SaveGameObject.Enable Gore?` _asbp_save_game_object))
    (set `self.Enable Aim Assist?` (`/Game/Gameplay/Framework/BP_SaveGameObject.Enable Aim Assist?` _asbp_save_game_object))
    ;;[1 1 1] Map/Level Unlock
    (set `self.Unlock Map 2` (`/Game/Gameplay/Framework/BP_SaveGameObject.Unlock Map 2` _asbp_save_game_object))
    (set `self.Unlock Level 2B` (`/Game/Gameplay/Framework/BP_SaveGameObject.Unlock Level 2B` _asbp_save_game_object))
    (set `self.Unlock Map 3` (`/Game/Gameplay/Framework/BP_SaveGameObject.Unlock Map 3` _asbp_save_game_object))
    (set `self.Unlock Level 3B` (`/Game/Gameplay/Framework/BP_SaveGameObject.Unlock Level 3B` _asbp_save_game_object))
    (return _output_get)))

(fn `Load SEM Player Data`
  (bind _returnvalue (`GameplayStatics.DoesSaveGameExist` "SEM Save 1"))
  (if _returnvalue
    (bind _returnvalue_2 (`GameplayStatics.LoadGameFromSlot` "SEM Save 1"))
    (bind _asbp_save_game_object (cast `/Game/Gameplay/Framework/BP_SaveGameObject` _returnvalue_2))
    (set `self.GI Coin Bank` (`/Game/Gameplay/Framework/BP_SaveGameObject.SEM Coin Bank` _asbp_save_game_object))
    (set `self.Unlocked Bully?` (`/Game/Gameplay/Framework/BP_SaveGameObject.Unlocked Bully?` _asbp_save_game_object))
    (set `self.Unlocked Heckler?` (`/Game/Gameplay/Framework/BP_SaveGameObject.Unlocked Heckler?` _asbp_save_game_object))
    (return)))

(fn `Save Player Data`
  (locals (`Player Ref` :type "/Game/Characters/Player/PlayerBP Object Reference"))
  (bind _player_data_coinbank (break `/Game/Gameplay/Framework/PlayerSaveData` (`/Game/Gameplay/Framework/BP_SaveGameObject.Player Data` (`self.Save Game Data`))))
  ;[1 1 1] Get Player & Write Data That Needs to be Saved to Save Game File
  (bind _asplayer_bp (cast `/Game/Characters/Player/PlayerBP` (`GameplayStatics.GetPlayerCharacter` 0)))
  (bind _output_get (set `local.Player Ref` _asplayer_bp))
  (set `/Game/Gameplay/Framework/BP_SaveGameObject.Player Data` (make `/Game/Gameplay/Framework/PlayerSaveData` (+ (`/Game/Characters/Player/PlayerBP.CoinsCollected` _output_get) _player_data_coinbank)) (`self.Save Game Data`))
  ;[1 1 1] Save File to Slot
  (`GameplayStatics.SaveGameToSlot` (`self.Save Game Data`) "SEM Save 1"))

(fn `Save SEM Game Data to Disk`
  (bind _returnvalue (`GameplayStatics.CreateSaveGameObject` "/Game/Gameplay/Framework/BP_SaveGameObject.BP_SaveGameObject_C"))
  (bind _asbp_save_game_object (cast `/Game/Gameplay/Framework/BP_SaveGameObject` _returnvalue))
  ;[1 1 1] Global Data
  (set `/Game/Gameplay/Framework/BP_SaveGameObject.SkipOpeningSequence?` (`self.SkipOpeningSequence?`) _asbp_save_game_object)
  (set `/Game/Gameplay/Framework/BP_SaveGameObject.Cell Shader Setting` (`self.Enable Cell Shader?`) _asbp_save_game_object)
  (set `/Game/Gameplay/Framework/BP_SaveGameObject.EnableHaptics?` (`self.EnableHaptics?`) _asbp_save_game_object)
  (set `/Game/Gameplay/Framework/BP_SaveGameObject.Input Sensitivity Override` (`self.Input Sensitivity Override`) _asbp_save_game_object)
  (set `/Game/Gameplay/Framework/BP_SaveGameObject.Enable Gore?` (`self.Enable Gore?`) _asbp_save_game_object)
  (set `/Game/Gameplay/Framework/BP_SaveGameObject.Enable Aim Assist?` (`self.Enable Aim Assist?`) _asbp_save_game_object)
  ;[1 1 1] Level Data
  (set `/Game/Gameplay/Framework/BP_SaveGameObject.Unlock Level 1B` (`self.Unlock Level 1B`) _asbp_save_game_object)
  (set `/Game/Gameplay/Framework/BP_SaveGameObject.Unlock Map 2` (`self.Unlock Map 2`) _asbp_save_game_object)
  (set `/Game/Gameplay/Framework/BP_SaveGameObject.Unlock Level 2B` (`self.Unlock Level 2B`) _asbp_save_game_object)
  (set `/Game/Gameplay/Framework/BP_SaveGameObject.Unlock Map 3` (`self.Unlock Map 3`) _asbp_save_game_object)
  (set `/Game/Gameplay/Framework/BP_SaveGameObject.Unlock Level 3B` (`self.Unlock Level 3B`) _asbp_save_game_object)
  (`GameplayStatics.SaveGameToSlot` _asbp_save_game_object "SEM Save 1"))

(fn `Save SEM Player Data to Disk`
  (bind _returnvalue (`GameplayStatics.CreateSaveGameObject` "/Game/Gameplay/Framework/BP_SaveGameObject.BP_SaveGameObject_C"))
  (bind _asbp_save_game_object (cast `/Game/Gameplay/Framework/BP_SaveGameObject` _returnvalue))
  (set `/Game/Gameplay/Framework/BP_SaveGameObject.SEM Coin Bank` (`self.GI Coin Bank`) _asbp_save_game_object)
  (set `/Game/Gameplay/Framework/BP_SaveGameObject.Unlocked Bully?` (`self.Unlocked Bully?`) _asbp_save_game_object)
  (set `/Game/Gameplay/Framework/BP_SaveGameObject.Unlocked Heckler?` (`self.Unlocked Heckler?`) _asbp_save_game_object)
  (`GameplayStatics.SaveGameToSlot` _asbp_save_game_object "SEM Save 1"))

(fn `Save Workshop Data`
  (bind _returnvalue (`|CreateWidget` "/Game/UI/UI_Assets/UIBlueprints/WB_Workshop.WB_Workshop_C" (`GameplayStatics.GetPlayerController` 0) null))
  (bind _aswb_workshop (cast `/Game/UI/UI_Assets/UIBlueprints/WB_Workshop` _returnvalue))
  (set `/Game/Gameplay/Framework/BP_SaveGameObject.Player Data` (make `/Game/Gameplay/Framework/PlayerSaveData` 0 false false false 0.0 0.0 0.0 false (`/Game/UI/UI_Assets/UIBlueprints/WB_Workshop.Purchased Bully?` _aswb_workshop)) (`self.Save Game Data`))
  ;[1 1 1] Save File to Slot
  (`GameplayStatics.SaveGameToSlot` (`self.Save Game Data`) "SEM Save 1"))