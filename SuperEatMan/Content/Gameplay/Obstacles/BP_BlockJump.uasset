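; BP_BlockJump is an obstacle that rewards or penalizes the player through two trigger colliders.
; Overlapping ScoreJumpCollider adds score, while overlapping BoxCollider subtracts score and one Health, then disables the actor's collision.
; Neither overlap checks the other actor; both always modify player 0's PlayerBP and print the updated values as debug text.
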(event `self.ScoreJumpCollider.OnComponentBeginOverlap`
  (params (OverlappedComponent :type "PrimitiveComponent Object Reference") (OtherActor :type "Actor Object Reference") (OtherComp :type "PrimitiveComponent Object Reference") (OtherBodyIndex :type Integer) (bFromSweep :type Boolean) (SweepResult :type "HitResult Structure (by ref)"))
  (`self.ScoreIncrease`))

(event `self.BoxCollider.OnComponentBeginOverlap`
  (params (OverlappedComponent :type "PrimitiveComponent Object Reference") (OtherActor :type "Actor Object Reference") (OtherComp :type "PrimitiveComponent Object Reference") (OtherBodyIndex :type Integer) (bFromSweep :type Boolean) (SweepResult :type "HitResult Structure (by ref)"))
  (`self.ScoreDecrease`))

(fn `ScoreDecrease`
  (returns (ScoreUpdate :type Integer))
  (bind _asplayer_bp (cast `/Game/Characters/Player/PlayerBP/PlayerBP` (`GameplayStatics.GetPlayerCharacter` 0)))
  (bind _output_get (set `/Game/Characters/Player/PlayerBP/PlayerBP.Score` (- (`/Game/Characters/Player/PlayerBP/PlayerBP.Score` _asplayer_bp) 50) _asplayer_bp))
  (`KismetSystemLibrary.PrintString` (`KismetStringLibrary.Conv_IntToString` _output_get))
  (`self.SetActorEnableCollision` false)
  (`self.SetActorEnableCollision` (`ActorComponent.GetOwner` (`self.ScoreJumpCollider`)) false)
  (bind _output_get_2 (set `/Game/Characters/Player/PlayerBP/PlayerBP.Health` (- (`/Game/Characters/Player/PlayerBP/PlayerBP.Health` _asplayer_bp) 1) _asplayer_bp))
  (`KismetSystemLibrary.PrintString` (`KismetStringLibrary.Conv_IntToString` _output_get_2) true true (struct :`R` 1.0 :`G` 0.007843 :`A` 1.0))
  (return _output_get_2))

(fn `ScoreIncrease`
  (returns (ScoreUpdate :type Integer))
  (bind _asplayer_bp (cast `/Game/Characters/Player/PlayerBP/PlayerBP` (`GameplayStatics.GetPlayerCharacter` 0)))
  (bind _output_get (set `/Game/Characters/Player/PlayerBP/PlayerBP.Score` (+ (`/Game/Characters/Player/PlayerBP/PlayerBP.Score` _asplayer_bp) 100) _asplayer_bp))
  (`KismetSystemLibrary.PrintString` (`KismetStringLibrary.Conv_IntToString` _output_get) true true (struct :`G` 0.074162 :`B` 1.0 :`A` 1.0))
  (return _output_get))

(fn `UserConstructionScript`)