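; Spline rail that carries a referenced boss actor, expected to be BP_Pylonator, from first to last point, snapping it to the start on construction.
; StartBoss scales the timeline play rate by spline length and the player's max movement speed, then plays it.
; Timeline updates set location and tangent-based rotation, with yaw turned 180 degrees to face back along the path.
; Separate hooks play or stop the timeline and store its playback position.
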(event `self.ReceiveBeginPlay`
  ;[1 1 1] Boss Ref
  (cast `/Game/Characters/NPC/Pylonator/BP_Pylonator` (`self.Actor`))
  (bind _asplayer_bp (cast `/Game/Characters/Player/PlayerBP` (`GameplayStatics.GetPlayerCharacter` 0)))
  (set `self.PlayerBPRef` _asplayer_bp))

(event `StartBoss`
  ;[1 1 1] Start Boss
  (`TimelineComponent.SetPlayRate` (`self.Timeline`) (/ 1.0 (/ (`SplineComponent.GetSplineLength` (`self.Spline`)) (`MovementComponent.GetMaxSpeed` (`Character.CharacterMovement` (`self.PlayerBPRef`))))))
  (`self.Play Timeline`))

(event `Play Timeline`
  ;[1 1 1] Start & Stop Timeline
  (`TimelineComponent.Play` (`self.Timeline`)))

(event `StopTimeline`
  ;[1 1 1] Start & Stop Timeline
  (`TimelineComponent.Stop` (`self.Timeline`)))

(fn `StorePlaybackPosition`
  (set `self.PlaybackPosition` (`TimelineComponent.GetPlaybackPosition` (`self.Timeline`))))

(fn `UserConstructionScript`
  (`self.K2_SetActorLocation` (`self.Actor`) (`SplineComponent.GetLocationAtSplinePoint` (`self.Spline`) 0 "World") false false))