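; BP_FoodDelivery is a food delivery collectible that tracks whether it has been picked up and carries a tip value.
; Overlap calls the parent handler, then marks it Collected once when PlayerHit is set.
; GivePlayerCoins adds the tips of all collected deliveries in the level to TotalTips, but only checks the player cast without awarding coins.
; Logic for attaching to the player's RocketFork is left disconnected.
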(event `self.ReceiveActorBeginOverlap`
  (params (OtherActor :type "Actor Object Reference"))
  (`parent.ReceiveActorBeginOverlap` OtherActor)
  (if (`self.PlayerHit`)
    (`/Engine/EditorBlueprintResources/StandardMacros.DoOnce` false
      (:`Completed`
        (set `self.Collected` true)))))

(event `self.AfterPickup`
  (`parent.AfterPickup`))

(fn `Give Player Coins`
  (locals (TotalTips :type Integer))
  (bind _outactors (`GameplayStatics.GetAllActorsOfClass` "BP_FoodDelivery_C"))
  (for _array_element _outactors
    (if (`/Game/Gameplay/Collectibles/FoodDelivery/BP_FoodDelivery.Collected` _array_element)
      (set `local.TotalTips` (+ (`/Game/Gameplay/Collectibles/FoodDelivery/BP_FoodDelivery.Tips` _array_element) (`local.TotalTips`)))))
  (cast `/Game/Characters/Player/PlayerBP` (`GameplayStatics.GetPlayerCharacter` 0)
    (:`then`
      (return))
    (:`CastFailed`
      (`KismetSystemLibrary.PrintString` "Not the player"))))

(fn `UserConstructionScript`
  (`parent.UserConstructionScript`))