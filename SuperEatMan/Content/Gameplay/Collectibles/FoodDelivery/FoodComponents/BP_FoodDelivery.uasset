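; A food delivery collectible that pays its Tips into the player's DeliveryCoins when picked up.
; On overlap, after the parent's handling, a PlayerHit check plays the pickup sound, then a DoOnce adds the coins and destroys the actor.
; A separate GivePlayerCoins function totals Tips across all BP_FoodDelivery actors, prints and returns the sum, and leaves its player cast unreached.
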(event `self.ReceiveActorBeginOverlap`
  (params (OtherActor :type "Actor Object Reference"))
  (bind _player (`self.Player`))
  (`parent.ReceiveActorBeginOverlap` OtherActor)
  (if (`self.PlayerHit`)
    (`GameplayStatics.PlaySound2D` "/Game/Sound/SFX/HealPickup.HealPickup" 1.0 1.0 0.0 null null)
    (`/Engine/EditorBlueprintResources/StandardMacros.DoOnce` false
      (:`Completed`
        (set `/Game/Characters/Player/PlayerBP.DeliveryCoins` (+ (`/Game/Characters/Player/PlayerBP.DeliveryCoins` _player) (`self.Tips`)) _player)
        (`self.K2_DestroyActor`)))))

(fn `Give Player Coins`
  (returns (Coins :type Integer))
  (locals (TotalTips :type Integer))
  (bind _totaltips (`local.TotalTips`))
  (bind _outactors (`GameplayStatics.GetAllActorsOfClass` "BP_FoodDelivery_C"))
  (for _array_element _outactors
    (if true
      (set `local.TotalTips` (+ (`/Game/Gameplay/Collectibles/FoodDelivery/FoodComponents/BP_FoodDelivery.Tips` _array_element) (`local.TotalTips`)))))
  (`KismetSystemLibrary.PrintString` (`KismetStringLibrary.Conv_IntToString` _totaltips))
  (return _totaltips))

(fn `UserConstructionScript`
  (`parent.UserConstructionScript`))