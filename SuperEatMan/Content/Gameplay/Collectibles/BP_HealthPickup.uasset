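; Health pickup collectible that adds health to the player on overlap, then destroys itself.
; The overlap event runs the parent's logic first, then checks PlayerHit before adding HealthGiven to the player's Health, with no clamp in this Blueprint.
; It then fires AfterPickup, which calls the parent version and destroys the actor.
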(event `self.ReceiveActorBeginOverlap`
  (params (OtherActor :type "Actor Object Reference"))
  (bind _player (`self.Player`))
  (`parent.ReceiveActorBeginOverlap` OtherActor)
  (if (`self.PlayerHit`)
    (set `/Game/Characters/Player/PlayerBP.Health` (+ (`/Game/Characters/Player/PlayerBP.Health` _player) (`self.HealthGiven`)) _player)
    (`self.AfterPickup`)))

(event `self.AfterPickup`
  (`parent.AfterPickup`)
  (`self.K2_DestroyActor`))

(fn `UserConstructionScript`
  (`parent.UserConstructionScript`))