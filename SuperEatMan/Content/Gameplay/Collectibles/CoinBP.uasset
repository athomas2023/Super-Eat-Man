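; CoinBP is a collectible coin that spins every Tick and is picked up when the player overlaps its sphere.
; Pickup adds CoinValue to the player's CoinsCollected and CoinStylePoints to SEMScore, plays a 2D sound and destroys the coin.
; TipMultiplier scales CoinValue by the RankStatus of the player reference cached at BeginPlay, but its rank-up binding is disconnected and never runs.
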(event `self.ReceiveBeginPlay`
  (bind _asplayer_bp (cast `/Game/Characters/Player/PlayerBP` (`GameplayStatics.GetPlayerCharacter` 0)))
  (set `self.As Player BP` _asplayer_bp))

(event `TipMultiplier`
  (switch `int` (`/Game/Characters/Player/PlayerBP.Rank Status` (`self.As Player BP`))
    (:`1`
      (set `self.Coin Value` 10))
    (:`2`
      (set `self.Coin Value` 15))
    (:`3`
      (set `self.Coin Value` 25))
    (:`4`
      (set `self.Coin Value` 30))
    (:`5`
      (set `self.Coin Value` 40))
    (:`6`
      (set `self.Coin Value` 50))))

(event `self.ReceiveTick`
  (params (DeltaSeconds :type "Float (single-precision)"))
  ;[1 1 1] Rotate Coin - Chnage to Timeline
  (`self.K2_AddActorLocalRotation` (struct :`Yaw` 3.0)))

(event `self.Sphere.OnComponentBeginOverlap`
  (params (OverlappedComponent :type "PrimitiveComponent Object Reference") (OtherActor :type "Actor Object Reference") (OtherComp :type "PrimitiveComponent Object Reference") (OtherBodyIndex :type Integer) (bFromSweep :type Boolean) (SweepResult :type "HitResult Structure (by ref)"))
  (bind _as_player_bp (`self.As Player BP`))
  ;[1 1 1] ++ Coins
  (if (== OtherActor _as_player_bp)
    (set `/Game/Characters/Player/PlayerBP.CoinsCollected` (+ (`/Game/Characters/Player/PlayerBP.CoinsCollected` _as_player_bp) (`self.Coin Value`)) _as_player_bp)
    ;[1 1 1] ++ Score
    (set `/Game/Characters/Player/PlayerBP.SEM Score` (+ (`/Game/Characters/Player/PlayerBP.SEM Score` _as_player_bp) (`self.Coin Style Points`)) _as_player_bp)
    (`GameplayStatics.PlaySound2D` "/Game/Sound/SFX/CoinPickup.CoinPickup" 1.0 1.0 0.0 null null)
    (`self.K2_DestroyActor`)))

(fn `UserConstructionScript`)