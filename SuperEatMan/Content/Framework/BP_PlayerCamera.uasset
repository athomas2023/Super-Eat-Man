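; BP_PlayerCamera is a standalone player camera that follows the player character.
; On BeginPlay it caches player controller 0 and casts the player character to PlayerBP.
; Every tick it sets itself as the controller's view target and moves its SpringArm to the world transform of the player's CameraTarget, with no sweep or interpolation in the graph.
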(event `self.ReceiveBeginPlay`
  (bind _asplayer_controller (cast `PlayerController` (`GameplayStatics.GetPlayerController` 0)))
  (set `self.As Player Controller` _asplayer_controller)
  (bind _asplayer_bp (cast `/Game/BluePrintResources/PlayerBP/PlayerBP` (`GameplayStatics.GetPlayerCharacter` 0)))
  (set `self.As Player BP` _asplayer_bp))

(event `self.ReceiveTick`
  (params (DeltaSeconds :type "Float (single-precision)"))
  (`PlayerController.SetViewTargetWithBlend` (`self.As Player Controller`) self 0.0 "VTBlend_Linear" 0.0 false)
  (`SceneComponent.K2_SetWorldTransform` (`self.SpringArm`) (`SceneComponent.K2_GetComponentToWorld` (`/Game/BluePrintResources/PlayerBP/PlayerBP.Camera Target` (`self.As Player BP`))) false false))

(fn `UserConstructionScript`)