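; Game instance that manages save slots and persists the player's coin count through BP_SaveGame1.
; LoadGame loads the named slot or creates a new save object, caching both slot name and object.
; SavePlayerData adds PlayerBP's collected coins to the banked total, resets other PlayerData fields to defaults, and writes the slot.
; LoadPlayerData copies the bank into the player's collected coins, while ClearSaveData deletes the slot.
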(event `Load Game`
  (params (`Save Slot Name` :type String))
  ;[1 1 1] Check for Selected File (Save Slot Name) in Save Game Object Folder
  (bind _output_get (set `self.Save Slot Name` `Save Slot Name`))
  (bind _returnvalue (`GameplayStatics.DoesSaveGameExist` _output_get))
  (if _returnvalue
    ;[1 1 1] If False: Creates Object and Set Local Ref
    ; If True: Load & Cast, then Set Local Ref
    (bind _returnvalue_2 (`GameplayStatics.LoadGameFromSlot` (`self.Save Slot Name`)))
    (bind _asbp_save_game_1 (cast `/Game/Framework/BP_SaveGame1` _returnvalue_2))
    (set `self.Save Game Data` _asbp_save_game_1)
    (else
      (bind _returnvalue_3 (`GameplayStatics.CreateSaveGameObject` "/Game/Framework/BP_SaveGame1.BP_SaveGame1_C"))
      (set `self.Save Game Data` _returnvalue_3))))

(event `self.ReceiveInit`)

(fn `Clear Save Data`
  (`GameplayStatics.DeleteGameInSlot` (`self.Save Slot Name`)))

(fn `Load Player Data`
  (locals (`Player Ref` :type "/Game/BluePrintResources/PlayerBP/PlayerBP Object Reference"))
  (bind _player_data_coinbank (break `/Game/Framework/PlayerSaveData` (`/Game/Framework/BP_SaveGame1.Player Data` (`self.Save Game Data`))))
  (bind _asplayer_bp (cast `/Game/BluePrintResources/PlayerBP/PlayerBP` (`GameplayStatics.GetPlayerCharacter` 0)))
  (bind _output_get (set `local.Player Ref` _asplayer_bp))
  (set `/Game/BluePrintResources/PlayerBP/PlayerBP.CoinsCollected` _player_data_coinbank _output_get))

(fn `Save Player Data`
  (locals (`Player Ref` :type "/Game/BluePrintResources/PlayerBP/PlayerBP Object Reference"))
  (bind _player_data_coinbank (break `/Game/Framework/PlayerSaveData` (`/Game/Framework/BP_SaveGame1.Player Data` (`self.Save Game Data`))))
  ;[1 1 1] Get Player and Copy "Coins Collected" to Save Game Object (File)
  (bind _asplayer_bp (cast `/Game/BluePrintResources/PlayerBP/PlayerBP` (`GameplayStatics.GetPlayerCharacter` 0)))
  (bind _output_get (set `local.Player Ref` _asplayer_bp))
  (set `/Game/Framework/BP_SaveGame1.Player Data` (make `/Game/Framework/PlayerSaveData` (+ (`/Game/BluePrintResources/PlayerBP/PlayerBP.CoinsCollected` _output_get) _player_data_coinbank)) (`self.Save Game Data`))
  ;[1 1 1] Take File and Save to Project Save File Folder
  (`GameplayStatics.SaveGameToSlot` (`self.Save Game Data`) (`self.Save Slot Name`)))