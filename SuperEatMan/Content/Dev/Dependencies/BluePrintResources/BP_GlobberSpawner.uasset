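; BP_GlobberSpawner is a spawner actor that endlessly spawns batches of a configurable enemy class at its own transform.
; BeginPlay triggers the SpawnEnemy event, which spawns NumberOfEnemies actors of EnemyType at once, waits SpawnDelay, then calls itself again.
; The self-calling event acts as a repeating timer, with no stop condition or cap on total spawns.
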(event `self.ReceiveBeginPlay`
  (`self.Spawn Enemy` (`self.Enemy Type`) (`self.GetTransform`) (`self.Number Of Enemies`)))

(event `Spawn Enemy`
  (params (`Enemy Type` :type "Actor Class Reference") (SpawnTransform :type "Transform Structure") (`Number of Enemies` :type Integer))
  (for _ (range `Number of Enemies`)
    (`|SpawnActorFromClass` `Enemy Type` SpawnTransform "Undefined" "MultiplyWithRoot" null null))
  (`KismetSystemLibrary.Delay` (`self.Spawn Delay`))
  (`self.Spawn Enemy` (`self.Enemy Type`) (`self.GetTransform`) (`self.Number Of Enemies`)))

(fn `UserConstructionScript`)