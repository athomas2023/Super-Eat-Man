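; BP_LBEndGameTrigger is a level-end trigger that completes the level when the player overlaps its collider.
; BeginPlay caches the player and BP_NewGameInstance references.
; On overlap it adds collected coins to the game instance's bank and saves player data, pauses the game, unlocks Map 2 and saves game data, then shows the WB_LevelComplete widget.
; Several older save and level-complete chains remain disconnected and never run.
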(event `self.ReceiveBeginPlay`
  ;[1 1 1] Get Player Ref
  (bind _asplayer_bp (cast `/Game/Characters/Player/PlayerBP` (`GameplayStatics.GetPlayerCharacter` 0)))
  (set `self.Player BP Ref` _asplayer_bp)
  (bind _asbp_new_game_instance (cast `/Game/Gameplay/Framework/BP_NewGameInstance` (`GameplayStatics.GetGameInstance`)))
  (set `self.Game Instance Ref` _asbp_new_game_instance))

(event `self.Collider.OnComponentBeginOverlap`
  (params (OverlappedComponent :type "PrimitiveComponent Object Reference") (OtherActor :type "Actor Object Reference") (OtherComp :type "PrimitiveComponent Object Reference") (OtherBodyIndex :type Integer) (bFromSweep :type Boolean) (SweepResult :type "HitResult Structure (by ref)"))
  ;[1 1 1] Display Level Complete Screen
  (cast `/Game/Characters/Player/PlayerBP` OtherActor)
  (`self.Save Player Data`)
  (`GameplayStatics.SetGamePaused` true)
  (`self.Save Game Data`)
  (bind _returnvalue (`|CreateWidget` "/Game/UI/UI_Assets/UIBlueprints/WB_LevelComplete.WB_LevelComplete_C"))
  (`UserWidget.AddToViewport` _returnvalue 0))

(fn `Save Game Data`
  (bind _game_instance_ref (`self.Game Instance Ref`))
  (set `/Game/Gameplay/Framework/BP_NewGameInstance.Unlock Map 2` true _game_instance_ref)
  (`/Game/Gameplay/Framework/BP_NewGameInstance.Save SEM Game Data to Disk` _game_instance_ref))

(fn `Save Player Data`
  (bind _game_instance_ref (`self.Game Instance Ref`))
  (set `/Game/Gameplay/Framework/BP_NewGameInstance.GI Coin Bank` (+ (`/Game/Characters/Player/PlayerBP.CoinsCollected` (`self.Player BP Ref`)) (`/Game/Gameplay/Framework/BP_NewGameInstance.GI Coin Bank` (`self.Game Instance Ref`))) _game_instance_ref)
  (`/Game/Gameplay/Framework/BP_NewGameInstance.Save SEM Player Data to Disk` _game_instance_ref))

(fn `UserConstructionScript`)