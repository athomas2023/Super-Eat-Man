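; BP_AlignCamera is a trigger actor that turns the player character to face a set direction on entering its collider, apparently to align the camera.
; BeginPlay caches the player as a PlayerBP reference.
; On overlap, it casts the entering actor to PlayerBP and sets that pawn's root component world rotation from the Direction component's forward vector, without sweep or teleport.
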(event `self.ReceiveBeginPlay`
  ;[1 1 1] Get Player Ref
  (bind _asplayer_bp (cast `/Game/Characters/Player/PlayerBP` (`GameplayStatics.GetPlayerCharacter` 0)))
  (set `self.Player BP Ref` _asplayer_bp))

(event `self.Collider.OnComponentBeginOverlap`
  (params (OverlappedComponent :type "PrimitiveComponent Object Reference") (OtherActor :type "Actor Object Reference") (OtherComp :type "PrimitiveComponent Object Reference") (OtherBodyIndex :type Integer) (bFromSweep :type Boolean) (SweepResult :type "HitResult Structure (by ref)"))
  ;[1 1 1] Set Camera Rotation
  (bind _asplayer_bp (cast `/Game/Characters/Player/PlayerBP` OtherActor))
  (bind _output_get (set `self.Player BP Ref` _asplayer_bp))
  (`SceneComponent.K2_SetWorldRotation` (`Actor.RootComponent` _output_get) (`KismetMathLibrary.Conv_VectorToRotator` (`SceneComponent.GetForwardVector` (`self.Direction`))) false false))

(fn `UserConstructionScript`)