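; Checkpoint trigger actor that moves the player's spawn point to its own location.
; When a PlayerBP that is not ragdolling overlaps the Collider, it writes the trigger's transform to SpawnTransform on BP_NewGameMode.
; A separate SpawnGlobber function, not called within this Blueprint, uses a DoOnce to spawn a single BP_Globber at the trigger's transform.
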(event `self.ReceiveBeginPlay`
  ;[1 1 1] Get Globber Ref
)

(event `self.Collider.OnComponentBeginOverlap`
  (params (OverlappedComponent :type "PrimitiveComponent Object Reference") (OtherActor :type "Actor Object Reference") (OtherComp :type "PrimitiveComponent Object Reference") (OtherBodyIndex :type Integer) (bFromSweep :type Boolean) (SweepResult :type "HitResult Structure (by ref)"))
  (bind _asplayer_bp (cast `/Game/Characters/Player/PlayerBP` OtherActor))
  (if (not (`/Game/Characters/Player/PlayerBP.Ragdolling` _asplayer_bp))
    (bind _asbp_new_game_mode (cast `/Game/Gameplay/Framework/BP_NewGameMode` (`GameplayStatics.GetGameMode`)))
    (set `/Game/Gameplay/Framework/BP_NewGameMode.Spawn Transform` (`self.GetTransform`) _asbp_new_game_mode)))

(fn `Spawn Globber`
  (`/Engine/EditorBlueprintResources/StandardMacros.DoOnce` false
    (:`Completed`
      (`|SpawnActorFromClass` "/Game/Characters/NPC/Enemies_Bot/Models/EnemyDrone/BP_Globber.BP_Globber_C" (`self.GetTransform`) "AlwaysSpawn" "MultiplyWithRoot" null null))))

(fn `UserConstructionScript`)