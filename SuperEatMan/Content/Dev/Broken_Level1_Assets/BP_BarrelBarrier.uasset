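; BP_BarrelBarrier is a destructible barrel obstacle that is removed when destroyed or hit by Wise Guy.
; DestroyCOne and DestroyBarrel simply destroy the actor.
; DamagedByWiseGuy also spawns the FX_WiseGuy effect at the actor's location and reports an obstacle, not an enemy, as destroyed.
; DamageTaken is empty, and the enemy health and GrindPoint nodes are disconnected leftovers that never run.
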(event `Destroy COne`
  ;[1 1 1] Death
  (`self.K2_DestroyActor`))

(event `Damage Taken`)

(fn `Damaged by Wise Guy`
  (returns (`Enemy Destroyed?` :type Boolean) (`Obstacle Destroyed?` :type Boolean))
  (`self.K2_DestroyActor`)
  (`NiagaraFunctionLibrary.SpawnSystemAtLocation` "/Game/Weapons/FX_WiseGuy.FX_WiseGuy" (`self.K2_GetActorLocation`))
  (return false true))

(fn `Destroy Barrel`
  (`self.K2_DestroyActor`))

(fn `UserConstructionScript`)