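; BP_BarrelBarrier_PR is a barrel obstacle that damages the player on contact.
; Its capsule overlap casts the other actor to PlayerBP and calls SEMDamaged.
; DestroyBarrel removes it, while DamagedByWiseGuy also spawns the Wise Guy effect and reports an obstacle, not an enemy, destroyed.
; DestroyCOne and DamageTaken are empty, and leftover enemy health and grind point logic never runs.
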(event `self.Capsule.OnComponentBeginOverlap`
  (params (OverlappedComponent :type "PrimitiveComponent Object Reference") (OtherActor :type "Actor Object Reference") (OtherComp :type "PrimitiveComponent Object Reference") (OtherBodyIndex :type Integer) (bFromSweep :type Boolean) (SweepResult :type "HitResult Structure (by ref)"))
  (bind _asplayer_bp (cast `/Game/Characters/Player/PlayerBP` OtherActor))
  (`/Game/Characters/Player/PlayerBP.SEM Damaged` _asplayer_bp))

(event `Destroy COne`
  ;[1 1 1] Death
)

(event `Damage Taken`)

(fn `Damaged by Wise Guy`
  (returns (`Enemy Destroyed?` :type Boolean) (`Obstacle Destroyed?` :type Boolean))
  (`self.K2_DestroyActor`)
  (`NiagaraFunctionLibrary.SpawnSystemAtLocation` "/Game/Weapons/FX_WiseGuy.FX_WiseGuy" (`self.K2_GetActorLocation`))
  (return false true))

(fn `Destroy Barrel`
  (`self.K2_DestroyActor`))

(fn `UserConstructionScript`)