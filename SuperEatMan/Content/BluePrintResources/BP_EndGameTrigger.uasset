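; BP_EndGameTrigger is a level-end trigger that saves player data and shows the level complete screen.
; On BeginPlay it caches the player character and the custom game instance.
; When any overlap with its Collider ends, a DoOnce calls SavePlayerData on the game instance, prints the result, pauses the game and adds WB_LevelComplete to the viewport.
; The overlapping actor is not checked, and the cached player reference is unused here.
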(event `self.ReceiveBeginPlay`
  ;[1 1 1] Get Player Ref
  (bind _asplayer_bp (cast `/Game/Characters/Player/PlayerBP` (`GameplayStatics.GetPlayerCharacter` 0)))
  (set `self.Player BP Ref` _asplayer_bp)
  (bind _asbp_new_game_instance (cast `/Game/Gameplay/Framework/BP_NewGameInstance` (`GameplayStatics.GetGameInstance`)))
  (set `self.Game Instance Ref` _asbp_new_game_instance))

(event `self.Collider.OnComponentEndOverlap`
  (params (OverlappedComponent :type "PrimitiveComponent Object Reference") (OtherActor :type "Actor Object Reference") (OtherComp :type "PrimitiveComponent Object Reference") (OtherBodyIndex :type Integer))
  ;[1 1 1] Display Level Complete Screen
  (`/Engine/EditorBlueprintResources/StandardMacros.DoOnce` false
    (:`Completed`
      (bind _get_coin_bank (`/Game/Gameplay/Framework/BP_NewGameInstance.Save Player Data` (`self.Game Instance Ref`)))
      (`KismetSystemLibrary.PrintString` (`KismetStringLibrary.Conv_IntToString` _get_coin_bank) true true (struct :`R` 1.0 :`G` 0.936701 :`A` 1.0))
      (`GameplayStatics.SetGamePaused` true)
      (bind _returnvalue (`|CreateWidget` "/Game/UI/UI_Assets/UIBlueprints/WB_LevelComplete.WB_LevelComplete_C"))
      (`UserWidget.AddToViewport` _returnvalue 0))))

(fn `UserConstructionScript`)