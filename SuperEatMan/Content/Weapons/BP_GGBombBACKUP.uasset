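; BP_GGBombBACKUP is a lobbed bomb projectile, apparently a backup, that damages the player on impact.
; On BeginPlay it sets its velocity with SuggestProjectileVelocityCustomArc toward the player's current position, without homing, and sets a lifespan.
; A sphere collider hit calls SEMDamaged on PlayerBP and destroys the bomb, as does taking damage.
; The author flags the lob as faulty, and the sauce-splat spawn is disconnected.
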(event `self.ReceiveBeginPlay`
  ;[1 0.03119 0.899] Lob Shot (will only work properly when GG is moving)
  ; Honestly just replace this code, something's wrong with it
  (bind _output_get (set `self.Start Position` (`self.K2_GetActorLocation` self)))
  (bind _outlaunchvelocity (`GameplayStatics.SuggestProjectileVelocity_CustomArc` _output_get (`self.K2_GetActorLocation` (`GameplayStatics.GetPlayerPawn` 0)) 0.0 0.9))
  (bind _output_get_2 (set `self.Velocity Vector` _outlaunchvelocity))
  (set `MovementComponent.Velocity` _output_get_2 (`self.ProjectileMovement`))
  (`self.SetLifeSpan` 30.0))

(event `self.Sphere Collider.OnComponentHit`
  (params (HitComponent :type "PrimitiveComponent Object Reference") (OtherActor :type "Actor Object Reference") (OtherComp :type "PrimitiveComponent Object Reference") (NormalImpulse :type "Vector Structure") (Hit :type "HitResult Structure (by ref)"))
  ;[1 0.03119 0.899] Set Destroy Self Here
  (`KismetSystemLibrary.PrintString` (`KismetSystemLibrary.GetDisplayName` OtherComp))
  (bind _asplayer_bp (cast `/Game/Characters/Player/PlayerBP` OtherActor)
    (:`then`
      (`/Game/Characters/Player/PlayerBP.SEM Damaged` _asplayer_bp))
    (:`CastFailed`
      _))
  (`self.K2_DestroyActor`))

(event `/Game/Characters/NPC/Enemies/I_Enemy.TakeDamage`
  (`self.K2_DestroyActor`))

(fn `UserConstructionScript`
  (bind _projectilemovement (`self.ProjectileMovement`))
  (set `ProjectileMovementComponent.InitialSpeed` (`self.Initial Speed`) _projectilemovement)
  (set `ProjectileMovementComponent.ProjectileGravityScale` (`self.Projectile Gravity Scale`) _projectilemovement))