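; Laser projectile that damages the player on impact.
; On BeginPlay it sets the ProjectileMovement velocity along its forward vector at LaserSpeed, then destroys itself after KillTime.
; A SphereCollider hit prints the hit component's name for debugging, calls SEMDamaged if the other actor is a PlayerBP, and destroys the projectile whatever it struck.
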(event `self.ReceiveBeginPlay`
  (bind _returnvalue (* (`self.GetActorForwardVector`) (`self.Laser Speed`)))
  ;[1 0.03119 0.899] Shoot forward
  (set `self.Velocity Vector` _returnvalue)
  (set `MovementComponent.Velocity` _returnvalue (`self.ProjectileMovement`))
  (`KismetSystemLibrary.Delay` (`self.KillTime`))
  (`self.K2_DestroyActor`))

(event `self.Sphere Collider.OnComponentHit`
  (params (HitComponent :type "PrimitiveComponent Object Reference") (OtherActor :type "Actor Object Reference") (OtherComp :type "PrimitiveComponent Object Reference") (NormalImpulse :type "Vector Structure") (Hit :type "HitResult Structure (by ref)"))
  ;[1 0.03119 0.899] Set Destroy Self Here
  (`KismetSystemLibrary.PrintString` (`KismetSystemLibrary.GetDisplayName` Hit_HitComponent))
  (bind _asplayer_bp (cast `/Game/Characters/Player/PlayerBP` OtherActor)
    (:`then`
      ;;[1 1 1] Damage Player
      (`/Game/Characters/Player/PlayerBP.SEM Damaged` _asplayer_bp))
    (:`CastFailed`
      _))
  (`self.K2_DestroyActor`))

(fn `UserConstructionScript`
  (`parent.UserConstructionScript`))