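; BP_ProjectileBase is a base projectile that lobs in an arc and leaves a sauce splat decal where it hits.
; The construction script feeds initial speed and gravity scale into ProjectileMovement.
; On BeginPlay, SuggestProjectileVelocityCustomArc sets the velocity toward a fixed distance along TargetActor's facing direction, not its location.
; On sphere collider hit, it spawns Decal_SauceSplat at the impact point and destroys itself.
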(event `self.ReceiveBeginPlay`
  ;[1 0.03119 0.899] Lob Shot
  (bind _output_get (set `self.Start Position` (`self.K2_GetActorLocation` self)))
  (bind _outlaunchvelocity (`GameplayStatics.SuggestProjectileVelocity_CustomArc` _output_get (+ _output_get (* (`KismetMathLibrary.Conv_RotatorToVector` (`self.K2_GetActorRotation` (`self.Target Actor`))) 3000.0))))
  (bind _output_get_2 (set `self.Velocity Vector` _outlaunchvelocity))
  (set `MovementComponent.Velocity` _output_get_2 (`self.ProjectileMovement`)))

(event `self.Sphere Collider.OnComponentHit`
  (params (HitComponent :type "PrimitiveComponent Object Reference") (OtherActor :type "Actor Object Reference") (OtherComp :type "PrimitiveComponent Object Reference") (NormalImpulse :type "Vector Structure") (Hit :type "HitResult Structure (by ref)"))
  ;[1 0.03119 0.899] Set Destroy Self Here
  (`|SpawnActorFromClass` "/Game/Assets/Decals/Decal_SauceSplat.Decal_SauceSplat_C" (`KismetMathLibrary.MakeTransform` Hit_Location) "Undefined" "MultiplyWithRoot" null null)
  (`self.K2_DestroyActor`))

(fn `UserConstructionScript`
  (bind _projectilemovement (`self.ProjectileMovement`))
  (set `ProjectileMovementComponent.InitialSpeed` (`self.Initial Speed`) _projectilemovement)
  (set `ProjectileMovementComponent.ProjectileGravityScale` (`self.Projectile Gravity Scale`) _projectilemovement))