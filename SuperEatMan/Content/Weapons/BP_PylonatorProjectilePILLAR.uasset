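; Pillar projectile for the Pylonator boss that damages the player on overlap and halts the boss's attack.
; It polls until the player stops ragdolling, then sets the boss spline timeline to its stored PlaybackPosition without firing events.
; It then destroys all other pillar and sweep projectiles in the level, followed by itself.
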(event `self.ReceiveActorBeginOverlap`
  (params (OtherActor :type "Actor Object Reference"))
  (bind _asplayer_bp (cast `/Game/Characters/Player/PlayerBP` OtherActor))
  (`/Game/Characters/Player/PlayerBP.SEM Damaged` _asplayer_bp)
  (bind _asbp_pylonator (cast `/Game/Characters/NPC/Pylonator/BP_Pylonator` (`self.GetOwner`)))
  (`/Game/Characters/NPC/Pylonator/BP_Pylonator.StopBossAttack` _asbp_pylonator)
  (if (`/Game/Characters/Player/PlayerBP.Ragdolling` _asplayer_bp) :!label _label
    (`KismetSystemLibrary.Delay` 0.2)
    (goto _label)
    (else
      (bind _outactors (`GameplayStatics.GetAllActorsOfClass` "/Game/Characters/NPC/Pylonator/BP_BossSpline.BP_BossSpline_C"))
      (bind _output (`|GetArrayItem` _outactors))
      (`TimelineComponent.SetPlaybackPosition` (`/Game/Characters/NPC/Pylonator/BP_BossSpline.Timeline` _output) (`/Game/Characters/NPC/Pylonator/BP_BossSpline.PlaybackPosition` _output) false true)
      (bind _outactors_2 (`GameplayStatics.GetAllActorsOfClass` "BP_PylonatorProjectilePILLAR_C"))
      (for _array_element _outactors_2
        (if (!= _array_element self)
          (`self.K2_DestroyActor` _array_element)))
      (bind _outactors_3 (`GameplayStatics.GetAllActorsOfClass` "/Game/Weapons/BP_PylonatorProjectileSWEEP.BP_PylonatorProjectileSWEEP_C"))
      (for _array_element_2 _outactors_3
        (if (!= _array_element_2 self)
          (`self.K2_DestroyActor` _array_element_2)))
      (`self.K2_DestroyActor`))))

(fn `UserConstructionScript`)