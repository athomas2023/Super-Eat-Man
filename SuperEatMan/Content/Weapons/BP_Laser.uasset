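; BP_Laser is a laser actor that projects a red Niagara beam along its forward vector.
; Each Tick it line traces on the Visibility channel over Distance, with debug drawing on, and sets the beam's end to the hit location or trace end.
; An impact effect moves to the hit location and shows only on a blocking hit.
; Unconnected nodes sketch an optional buildup effect that would grow Distance over time.
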(event `self.ReceiveBeginPlay`
  (`FXSystemComponent.SetColorParameter` (`self.Niagara Laser`) "Color" (struct :`R` 1.0 :`B` 0.029524 :`A` 1.0))
  (`FXSystemComponent.SetColorParameter` (`self.Niagara Laser Impact`) "Color" (struct :`R` 1.0 :`B` 0.029524 :`A` 1.0)))

(event `self.ReceiveTick`
  (params (DeltaSeconds :type "Float (single-precision)"))
  (bind _returnvalue (`self.K2_GetActorLocation`))
  (bind _output_get (set `self.Trace End` (+ _returnvalue (* (`self.GetActorForwardVector`) (`self.Distance`)))))
  (bind _outhit (`KismetSystemLibrary.LineTraceSingle` :`Start` _returnvalue :`End` _output_get :`TraceChannel` "TraceTypeQuery1" :`DrawDebugType` "ForOneFrame"))
  (set `self.Blocked Hit` (`GameplayStatics.BreakHitResult` _outhit))
  (set `self.Hit Location` (`.Location` (`GameplayStatics.BreakHitResult` _outhit)))
  (`FXSystemComponent.SetVectorParameter` (`self.Niagara Laser`) "LaserEnd" (select `bool` (`self.Blocked Hit`) :`false` (`self.Trace End`) :`true` (`self.Hit Location`)))
  (`SceneComponent.SetVisibility` (`self.Niagara Laser Impact`) (`self.Blocked Hit`) false)
  (`SceneComponent.K2_SetWorldLocation` (`self.Niagara Laser Impact`) (`self.Hit Location`) false false))

(fn `UserConstructionScript`)