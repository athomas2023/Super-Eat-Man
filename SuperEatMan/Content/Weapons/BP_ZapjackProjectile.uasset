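; Zapjack weapon projectile that fires a straight electric shot at the player and damages their SEM.
; On BeginPlay it sets its velocity toward player 0's current location at InitialSpeed, with no homing afterward.
; It plays a 2D electric sound that it toggles after a delay, and expires on a short lifespan.
; Sphere overlap with PlayerBP calls SEMDamaged without destroying the projectile.
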(event `self.ReceiveBeginPlay`
  ;[1 0.03119 0.899] Straight Shot
  ; Can be used to Track SEM and Shoot at a Faster or Slower Velocity Based on SEM Distance
  ; **Will need to handle how enemy tracks SEM per Enemy - Once Determined Passthrough with "Target Actor"
  (bind _asplayer_bp (cast `/Game/Characters/Player/PlayerBP` (`GameplayStatics.GetPlayerCharacter` 0)))
  (set `MovementComponent.Velocity` (* (`KismetMathLibrary.Normal` (- (`self.K2_GetActorLocation` _asplayer_bp) (`self.K2_GetActorLocation` self))) (`self.Initial Speed`)) (`self.ProjectileMovement`))
  (bind _returnvalue (`GameplayStatics.SpawnSound2D` "/Game/Sound/SFX/electric.electric" 1.0 1.0 0.0 null))
  (`self.SetLifeSpan` 5.0)
  (`KismetSystemLibrary.Delay` 3.0)
  (`ActorComponent.ToggleActive` _returnvalue))

(event `self.Sphere Collider.OnComponentBeginOverlap`
  (params (OverlappedComponent :type "PrimitiveComponent Object Reference") (OtherActor :type "Actor Object Reference") (OtherComp :type "PrimitiveComponent Object Reference") (OtherBodyIndex :type Integer) (bFromSweep :type Boolean) (SweepResult :type "HitResult Structure (by ref)"))
  (bind _asplayer_bp (cast `/Game/Characters/Player/PlayerBP` OtherActor))
  (`/Game/Characters/Player/PlayerBP.SEM Damaged` _asplayer_bp))

(fn `UserConstructionScript`
  (`parent.UserConstructionScript`))