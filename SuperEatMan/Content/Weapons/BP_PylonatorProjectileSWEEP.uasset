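; BP_PylonatorProjectileSWEEP is a sweep-attack projectile of the Pylonator boss that damages the player on overlap.
; A hit calls SEMDamaged on the PlayerBP, then clears BossAttacking on the owning BP_Pylonator.
; It then destroys all other SWEEP and PILLAR projectiles and itself, so one hit ends the attack.
; The cleanup only runs if the projectile's owner is a BP_Pylonator.
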(event `self.ReceiveActorBeginOverlap`
  (params (OtherActor :type "Actor Object Reference"))
  (bind _asplayer_bp (cast `/Game/Characters/Player/PlayerBP` OtherActor))
  (`/Game/Characters/Player/PlayerBP.SEM Damaged` _asplayer_bp)
  (bind _asbp_pylonator (cast `/Game/Characters/NPC/Pylonator/BP_Pylonator` (`self.GetOwner`)))
  (set `/Game/Characters/NPC/Pylonator/BP_Pylonator.BossAttacking` false _asbp_pylonator)
  (bind _outactors (`GameplayStatics.GetAllActorsOfClass` "BP_PylonatorProjectileSWEEP_C"))
  (for _array_element _outactors
    (if (!= _array_element self)
      (`self.K2_DestroyActor` _array_element)))
  (bind _outactors_2 (`GameplayStatics.GetAllActorsOfClass` "/Game/Weapons/BP_PylonatorProjectilePILLAR.BP_PylonatorProjectilePILLAR_C"))
  (for _array_element_2 _outactors_2
    (if (!= _array_element_2 self)
      (`self.K2_DestroyActor` _array_element_2)))
  (`self.K2_DestroyActor`))

(fn `UserConstructionScript`)