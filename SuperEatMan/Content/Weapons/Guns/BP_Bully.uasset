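; BP_Bully is the player's Bully gun, a child weapon with slug and birdshot fire modes, tuned by GameInstance upgrade mods.
; Both shots play effects and spend ammo; an empty magazine or player reload event triggers a delayed refill.
; Slugs use the parent trace, but the override forwards zero damage.
; Birdshot runs seven randomized traces but ignores their results, damaging TargetedActor each pass if it implements I_Enemy.
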(event `self.ReceiveBeginPlay`
  ;[1 1 1] Inherited
  (`parent.ReceiveBeginPlay`)
  (set `self.Current Magazine` (+ (`/Game/Gameplay/Framework/BP_NewGameInstance.BullyShotMod` (`self.BP New Game Instance Reference`)) (`self.Base Magazine Size`)))
  (set `self.Base Reload Delay` (- (`/Game/Gameplay/Framework/BP_NewGameInstance.BullyReloadMod` (`self.BP New Game Instance Reference`)) (`self.Base Reload Delay`)))
  (if (`/Game/Gameplay/Framework/BP_NewGameInstance.bBullyMod` (`self.BP New Game Instance Reference`))
    (set `self.WeaponRange` (`self.Bully Slug Fire Distance`))
    (set `self.Slug Base Damage` (`self.Bully Slug Damage`))
    (else
      (set `self.WeaponRange` (`self.Bird Shot Fire Distance`))
      (set `self.Bird Base Damage` (+ (`self.Bird Shot Damage`) (`/Game/Gameplay/Framework/BP_NewGameInstance.BullyDmgMod` (`self.BP New Game Instance Reference`))))))
  (add `self.OnMagazineEmpty` (delegate `Reload Bully`))
  (add `/Game/Characters/Player/PlayerBP.OnReload` (`self.Player BP Reference`) (delegate `Reload Bully`)))

(event `self.ReceiveTick`
  (params (DeltaSeconds :type "Float (single-precision)"))
  ;[1 1 1] Inherited
  (`parent.ReceiveTick` 0.0))

(event `Reload Bully`
  (bind _base_reload_delay (`self.Base Reload Delay`))
  ;[1 1 1] Reload
  (set `self.bIsReloading` true)
  (set `/Game/Characters/Player/PlayerBP.bReloading` true (`self.Player BP Reference`))
  (`KismetSystemLibrary.Delay` _base_reload_delay)
  (`KismetSystemLibrary.PrintString` "Bully Ready!" true true (struct :`G` 1.0 :`B` 0.133312 :`A` 1.0) _base_reload_delay)
  (set `self.Current Magazine` (`self.Base Magazine Size`))
  (set `self.bIsReloading` false)
  (set `/Game/Characters/Player/PlayerBP.bReloading` false (`self.Player BP Reference`))
  (`self.OnMagazineReloaded`))

(event `Shoot Slug`
  (if (`self.bIsReloading`)
    (`KismetSystemLibrary.PrintString` "Reloading Bully" true true (struct :`R` 1.0 :`B` 0.120504 :`A` 1.0) (`self.Base Reload Delay`))
    (else
      ;[1 1 1] SFX & VFX
      (`GameplayStatics.PlaySoundAtLocation` "/Game/Sound/SFX/Bully_shoot.Bully_shoot" (`SceneComponent.K2_GetComponentLocation` (`Character.CapsuleComponent` (`GameplayStatics.GetPlayerCharacter` 0))) (struct) 1.0 1.0 0.0 null null null null)
      (`NiagaraFunctionLibrary.SpawnSystemAtLocation` "/Game/Weapons/FX_WiseGuy.FX_WiseGuy" (`SceneComponent.K2_GetComponentLocation` (`/Game/Characters/Player/PlayerBP.Wiseguy Muzzle` (`self.Player BP Reference`))) (struct :`Roll` 90.0) (0.01 0.01 0.01))
      ;[1 1 1] Bullet Trace
      (`self.Shoot Weapon Trace` (`self.Bully Slug Fire Distance`) (`self.Slug Base Damage`))
      (`KismetSystemLibrary.PrintString` "Slug")
      ;[1 1 1] Cycling Rounds
      (bind _result (`/Engine/EditorBlueprintResources/StandardMacros.DecrementInt` (`self.Current Magazine`))
        (:`  `
          (if (<= _result 0)
            (`self.OnMagazineEmpty`)
            (else
              ;[1 1 1] Haptics
              (if (`self.Haptics Controller`)
                (`PlayerController.K2_ClientPlayForceFeedback` (`GameplayStatics.GetPlayerController` 0) "/Game/Gameplay/Input/HapticFeedback/FFE_Wiseguy.FFE_Wiseguy" "None" false false false)))))))))

(event `Shoot Bird Shot`
  (if (`self.bIsReloading`)
    (`KismetSystemLibrary.PrintString` "Reloading Bully" true true (struct :`R` 1.0 :`B` 0.120504 :`A` 1.0) (`self.Base Reload Delay`))
    (else
      ;[1 1 1] SFX & VFX
      (`GameplayStatics.PlaySoundAtLocation` "/Game/Sound/SFX/Bully_shoot.Bully_shoot" (`SceneComponent.K2_GetComponentLocation` (`Character.CapsuleComponent` (`GameplayStatics.GetPlayerCharacter` 0))) (struct) 1.0 1.0 0.0 null null null null)
      (`NiagaraFunctionLibrary.SpawnSystemAtLocation` "/Game/Weapons/FX_WiseGuy.FX_WiseGuy" (`SceneComponent.K2_GetComponentLocation` (`/Game/Characters/Player/PlayerBP.Wiseguy Muzzle` (`self.Player BP Reference`))) (struct :`Roll` 90.0) (0.01 0.01 0.01))
      (`self.FireBirdShot` (`self.Bird Base Damage`))
      (`KismetSystemLibrary.PrintString` "Bird" true true (struct :`R` 1.0 :`G` 0.070607 :`A` 1.0))
      ;[1 1 1] Cycling Rounds
      (bind _result (`/Engine/EditorBlueprintResources/StandardMacros.DecrementInt` (`self.Current Magazine`))
        (:`  `
          (if (<= _result 0)
            (`self.OnMagazineEmpty`)
            (else
              ;[1 1 1] Haptics
              (if (`self.Haptics Controller`)
                (`PlayerController.K2_ClientPlayForceFeedback` (`GameplayStatics.GetPlayerController` 0) "/Game/Gameplay/Input/HapticFeedback/FFE_Wiseguy.FFE_Wiseguy" "None" false false false)))))))))

(fn `FireBirdShot`
  (params (`Bird Base Damage` :type "Float (double-precision)"))
  (locals (Shootable :type "Array of EObjectTypeQuery Enum"))
  (bind _bulletspread (`self.BulletSpread`))
  (bind _bulletspread_2 (`self.BulletSpread`))
  (bind _bulletspread_3 (`self.BulletSpread`))
  (bind (_worldlocation _worlddirection) (`PlayerController.DeprojectMousePositionToWorld` (`GameplayStatics.GetPlayerController` 0)))
  (for _ (range 1 8)
    (bind _outhit (`KismetSystemLibrary.LineTraceSingleForObjects` (+ _worldlocation (* _worlddirection (`self.Bird Shot Fire Distance`)) (`KismetMathLibrary.MakeVector` (`KismetMathLibrary.RandomFloatInRange` (* _bulletspread_3 -1.0) _bulletspread_3) (`KismetMathLibrary.RandomFloatInRange` (* _bulletspread_2 -1.0) _bulletspread_2) (`KismetMathLibrary.RandomFloatInRange` (* _bulletspread -1.0) _bulletspread))) (`self.K2_GetActorLocation` (`self.Targeted Actor`)) (`local.Shootable`)))
    (if (`KismetSystemLibrary.DoesImplementInterface` (`self.Targeted Actor`) "/Game/Characters/NPC/Enemies/I_Enemy.I_Enemy_C")
      (message `/Game/Characters/NPC/Enemies/I_Enemy.TakeDamage` (`self.Targeted Actor`) `Bird Base Damage` (0.0 0.0 0.0))
      ;[1 1 1] Should be on Enemy
      (`self.OnHitEnemy`))))

(fn `Project Aim Assist Trace`
  (params (Distance :type "Float (double-precision)"))
  (returns (`Targeted Actor` :type "Actor Object Reference"))
  (bind _targeted_actor (`parent.Project Aim Assist Trace` Distance))
  (return _targeted_actor))

(fn `Shoot Weapon Trace`
  (params (`Bullet Distance` :type "Float (double-precision)") (BaseDamage :type "Float (double-precision)"))
  (locals (Shootable :type "Array of EObjectTypeQuery Enum"))
  (`parent.Shoot Weapon Trace` `Bullet Distance` 0.0))

(fn `UserConstructionScript`
  (`parent.UserConstructionScript`))