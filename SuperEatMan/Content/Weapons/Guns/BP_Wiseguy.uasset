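; BP_Wiseguy is a child weapon Blueprint for the Wiseguy gun, with single-shot and three-round burst fire.
; Each shot plays effects, runs the weapon trace, spawns a BP_Projectile and decrements the magazine, with optional controller rumble.
; An empty magazine or player reload event triggers a delayed refill that blocks firing.
; The trace override passes zero damage and multiplier to the parent, ignoring its inputs.
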(event `self.ReceiveBeginPlay`
  ;[1 1 1] Inherited
  (`parent.ReceiveBeginPlay`)
  (set `self.Current Magazine` (`self.Base Magazine Size`))
  (add `self.OnMagazineEmpty` (delegate `Reload Wiseguy`))
  (add `/Game/Characters/Player/PlayerBP.OnReload` (`self.Player BP Reference`) (delegate `Reload Wiseguy`)))

(event `self.ReceiveTick`
  (params (DeltaSeconds :type "Float (single-precision)"))
  ;[1 1 1] Inherited
  (`parent.ReceiveTick` 0.0))

(event `Reload Wiseguy`
  (bind _base_reload_delay (`self.Base Reload Delay`))
  ;[1 1 1] Reload Loop
  (set `self.bIsReloading` true)
  (`KismetSystemLibrary.Delay` _base_reload_delay)
  (`KismetSystemLibrary.PrintString` "Ready!" true true (struct :`G` 1.0 :`B` 0.133312 :`A` 1.0) _base_reload_delay)
  (set `self.Current Magazine` (`self.Base Magazine Size`))
  (set `self.bIsReloading` false)
  (`self.OnMagazineReloaded`))

(event `Shoot Wiseguy`
  ;[1 1 1] Check Can Shoot
  (if (`self.bIsReloading`)
    (`KismetSystemLibrary.PrintString` "Reloading..." true true (struct :`R` 1.0 :`B` 0.120504 :`A` 1.0) (`self.Base Reload Delay`))
    (else
      ;[1 1 1] SFX & VFX
      (`GameplayStatics.PlaySoundAtLocation` "/Game/Sound/SFX/Wiseguy_shoot.Wiseguy_shoot" (`SceneComponent.K2_GetComponentLocation` (`Character.CapsuleComponent` (`GameplayStatics.GetPlayerCharacter` 0))) (struct) 1.0 1.0 0.0 null null null null)
      (`NiagaraFunctionLibrary.SpawnSystemAtLocation` "/Game/Weapons/FX_WiseGuy.FX_WiseGuy" (`SceneComponent.K2_GetComponentLocation` (`/Game/Characters/Player/PlayerBP.Wiseguy Muzzle` (`self.Player BP Reference`))) (struct :`Roll` 90.0) (0.001 0.001 0.001))
      ;[1 1 1] Bullet Trace
      (`self.Shoot Weapon Trace` (`self.Wiseguy Fire Distance`) (`self.Base Damage`) (`self.Damage Multiplier`))
      ;[1 1 1] Projectile
      (`|SpawnActorFromClass` "/Game/Weapons/BP_Projectile.BP_Projectile_C" (`SceneComponent.K2_GetComponentToWorld` (`/Game/Characters/Player/PlayerBP.Wiseguy Muzzle` (`self.Player BP Reference`))) "Undefined" "MultiplyWithRoot" null null)
      (`KismetSystemLibrary.PrintString` "Wiseguy")
      ;[1 1 1] Cycle Rounds
      (bind _result (`/Engine/EditorBlueprintResources/StandardMacros.DecrementInt` (`self.Current Magazine`))
        (:`  `
          (if (<= _result 0)
            (`self.OnMagazineEmpty`)
            (else
              ;[1 1 1] Haptics
              (if (`self.Haptics Controller`)
                (`PlayerController.K2_ClientPlayForceFeedback` (`GameplayStatics.GetPlayerController` 0) "/Game/Gameplay/Input/HapticFeedback/FFE_Wiseguy.FFE_Wiseguy" "None" false false false)))))))))

(event `Wiseguy 3 Burst`
  ;[1 1 1] 3 Burst Mod
  (`/Engine/EditorBlueprintResources/StandardMacros.DoOnce` false :!label _label
    (:`Completed`
      (`self.Shoot Wiseguy`)
      (`KismetSystemLibrary.Delay` 0.11)
      (`self.Shoot Wiseguy`)
      (`KismetSystemLibrary.Delay` 0.11)
      (`self.Shoot Wiseguy`)
      (`KismetSystemLibrary.Delay` 0.5)
      (goto _label :!via `Reset`))))

(fn `Cycle Rounds`
  (params (Magazine :type Integer :default 0)))

(fn `Project Aim Assist Trace`
  (params (Distance :type "Float (double-precision)"))
  (returns (`Targeted Actor` :type "Actor Object Reference"))
  (bind _targeted_actor (`parent.Project Aim Assist Trace` Distance))
  (return _targeted_actor))

(fn `Shoot Weapon Trace`
  (params (`Bullet Distance` :type "Float (double-precision)") (BaseDamage :type "Float (double-precision)") (DamageMultiplier :type "Float (double-precision)"))
  (`parent.Shoot Weapon Trace` `Bullet Distance` 0.0 0.0)
  (return))

(fn `UserConstructionScript`
  (`parent.UserConstructionScript`))