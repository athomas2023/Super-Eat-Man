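; BP_Heckler is a child gun Blueprint for the Heckler weapon, a hitscan shot that destroys what it targets.
; While Heckler is equipped with aim assist on, Tick caches a target from the parent's AimAssist.
; Shoot plays laser sound and muzzle FX, then line-traces toward that target and destroys TargetedActor, or without assist traces along the mouse ray and destroys the hit actor.
; Grind-kill scoring is disconnected, pending rework.
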(event `self.ReceiveTick`
  (params (DeltaSeconds :type "Float (single-precision)"))
  (if (== (`/Game/Characters/Player/PlayerBP.Currently Equiped Weapon` (`self.Player BP Reference`)) (`self.Heckler Mode`))
    (if (`self.Enable Aim Assist?`)
      (bind _out_hit_hit_actor (`self.Aim Assist` (`self.Bullet Distance`)))
      (set `self.AA Target` _out_hit_hit_actor))))

(fn `Aim Assist`
  (params (Distance :type "Float (double-precision)") (`Fire Mode` :type Integer))
  (returns (`Out Hit Hit Actor` :type "Actor Object Reference"))
  (bind _out_hit_hit_actor (`parent.Aim Assist` Distance 0))
  (return _out_hit_hit_actor))

(fn `Shoot`
  (params (`Fire Mode` :type Integer))
  (locals (`Shootable Object Types` :type "Array of EObjectTypeQuery Enum") (`Object Types` :type "Array of EObjectTypeQuery Enum") (`SEM Score` :type "Float (double-precision)") (`Grind Kill` :type "Float (double-precision)"))
  (bind _aa_target (`self.AA Target`))
  (bind (_worldlocation _worlddirection) (`PlayerController.DeprojectMousePositionToWorld` (`GameplayStatics.GetPlayerController` 0)))
  ;[1 1 1] Heckler Fire Select
  (if (== `Fire Mode` (`self.Heckler Mode`))
    (`GameplayStatics.PlaySoundAtLocation` "/Game/Sound/SFX/Laser_pistol.Laser_pistol" (`SceneComponent.K2_GetComponentLocation` (`Character.CapsuleComponent` (`GameplayStatics.GetPlayerCharacter` 0))) (struct) 1.0 1.0 0.0 null null null null)
    (`NiagaraFunctionLibrary.SpawnSystemAtLocation` "/Game/Weapons/FX_WiseGuy.FX_WiseGuy" (`SceneComponent.K2_GetComponentLocation` (`/Game/Characters/Player/PlayerBP.Wiseguy Muzzle` (`self.Player BP Reference`))) (struct :`Roll` 90.0) (0.01 0.01 0.01))
    (if (`self.Enable Aim Assist?`)
      (`/Engine/EditorBlueprintResources/StandardMacros.IsValid` _aa_target
        (:`Is Valid`
          (bind _outhit (`KismetSystemLibrary.LineTraceSingleForObjects` :`Start` _worldlocation :`End` (`self.K2_GetActorLocation` _aa_target) :`ObjectTypes` (`local.Shootable Object Types`) :`DrawTime` 1.0))
          (`GameplayStatics.PlaySoundAtLocation` "/Game/Sound/SFX/RobotDamaged.RobotDamaged" (`.Location` (`GameplayStatics.BreakHitResult` _outhit)) (struct) 1.0 1.0 0.0 null null null null)
          (`self.K2_DestroyActor` (`self.Targeted Actor`))))
      (else
        (bind _outhit_2 (`KismetSystemLibrary.LineTraceSingleForObjects` :`Start` _worldlocation :`End` (+ _worldlocation (* _worlddirection (`self.Bullet Distance`))) :`ObjectTypes` (`local.Shootable Object Types`) :`DrawTime` 1.0))
        (bind (_bblockinghit _binitialoverlap _time _distance _location _impactpoint _normal _impactnormal _physmat _hitactor) (`GameplayStatics.BreakHitResult` _outhit_2))
        (`/Engine/EditorBlueprintResources/StandardMacros.IsValid` _hitactor
          (:`Is Valid`
            (`GameplayStatics.PlaySoundAtLocation` "/Game/Sound/SFX/RobotDamaged.RobotDamaged" _location (struct) 1.0 1.0 0.0 null null null null)
            (`self.K2_DestroyActor` _hitactor)))))))

(fn `UserConstructionScript`
  (`parent.UserConstructionScript`))