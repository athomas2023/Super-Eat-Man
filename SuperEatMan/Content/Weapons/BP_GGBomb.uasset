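; BP_GGBomb is a bomb projectile lobbed in an arc at the player's position when it spawns.
; On BeginPlay it sets its launch velocity with SuggestProjectileVelocityCustomArc, which an author note flags as faulty.
; Tick triggers Explode based on an X-axis comparison with the player, damaging them within KillRange.
; Collisions destroy it, damaging PlayerBP if hit, and TakeDamage destroys it once BombHits runs out.
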(event `self.ReceiveBeginPlay`
  ;[1 0.03119 0.899] Lob Shot (will only work properly when GG is moving)
  ; Honestly just replace this code, something's wrong with it
  (bind _output_get (set `self.Start Position` (`self.K2_GetActorLocation` self)))
  (bind _outlaunchvelocity (`GameplayStatics.SuggestProjectileVelocity_CustomArc` _output_get (`SceneComponent.K2_GetComponentLocation` (`Character.Mesh` (`GameplayStatics.GetPlayerCharacter` 0))) 0.0 0.75))
  (bind _output_get_2 (set `self.Velocity Vector` _outlaunchvelocity))
  (set `MovementComponent.Velocity` _output_get_2 (`self.ProjectileMovement`))
  (`self.SetLifeSpan` 30.0))

(event `self.ReceiveTick`
  (params (DeltaSeconds :type "Float (single-precision)"))
  (bind _returnvalue_x (`KismetMathLibrary.BreakVector` (`SceneComponent.K2_GetComponentLocation` (`self.Sphere Collider`))))
  (bind _returnvalue_x_2 (`KismetMathLibrary.BreakVector` (`SceneComponent.K2_GetComponentLocation` (`Character.Mesh` (`GameplayStatics.GetPlayerCharacter` 0)))))
  (if (>= _returnvalue_x_2 (- _returnvalue_x (`self.Explode Window`)))
    (`KismetSystemLibrary.PrintString` "BOOM")
    (`self.Explode`)))

(event `self.Sphere Collider.OnComponentHit`
  (params (HitComponent :type "PrimitiveComponent Object Reference") (OtherActor :type "Actor Object Reference") (OtherComp :type "PrimitiveComponent Object Reference") (NormalImpulse :type "Vector Structure") (Hit :type "HitResult Structure (by ref)"))
  ;[1 0.03119 0.899] Set Destroy Self Here
  (`KismetSystemLibrary.PrintString` (`KismetSystemLibrary.GetDisplayName` OtherComp))
  (bind _asplayer_bp (cast `/Game/Characters/Player/PlayerBP` OtherActor)
    (:`then`
      (`/Game/Characters/Player/PlayerBP.SEM Damaged` _asplayer_bp))
    (:`CastFailed`
      _))
  (`self.K2_DestroyActor`))

(event `Explode`
  (bind _returnvalue (`KismetMathLibrary.VSize` (- (`SceneComponent.K2_GetComponentLocation` (`Character.Mesh` (`GameplayStatics.GetPlayerCharacter` 0))) (`self.K2_GetActorLocation`))))
  ;[1 1 1] Boom
  (`KismetSystemLibrary.PrintString` (`KismetStringLibrary.Conv_DoubleToString` _returnvalue))
  (if (<= _returnvalue (`self.KillRange`))
    (bind _asplayer_bp (cast `/Game/Characters/Player/PlayerBP` (`GameplayStatics.GetPlayerCharacter` 0))
      (:`then`
        (`/Game/Characters/Player/PlayerBP.SEM Damaged` _asplayer_bp))
      (:`CastFailed`
        (`KismetSystemLibrary.PrintString` "Error - where is SEM"))))
  (`self.K2_DestroyActor`))

(event `/Game/Characters/NPC/Enemies/I_Enemy.TakeDamage`
  (params (BaseDamage :type "Float (double-precision)") (ImpactLocation :type "Vector Structure"))
  (bind _result (`/Engine/EditorBlueprintResources/StandardMacros.DecrementInt` (`self.BombHits`))
    (:`  `
      (if (<= _result 0)
        (`self.K2_DestroyActor`)))))

(fn `UserConstructionScript`
  (bind _projectilemovement (`self.ProjectileMovement`))
  (set `ProjectileMovementComponent.InitialSpeed` (`self.Initial Speed`) _projectilemovement)
  (set `ProjectileMovementComponent.ProjectileGravityScale` (`self.Projectile Gravity Scale`) _projectilemovement))